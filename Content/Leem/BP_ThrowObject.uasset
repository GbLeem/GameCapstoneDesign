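; BP_ThrowObject is a thrown object that reports hits to characters and expires after a limited lifetime.
; Each tick it sphere-traces a short distance ahead of its Collision sphere along that component's velocity, using a slightly reduced radius.
; If the hit actor is a BP_CharacterBase, it calls OnHit with the bone and inverted horizontal normal, then destroys itself.
; A Life countdown also destroys it when it runs out.
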(event EventBeginPlay)

(event Collision|EventActorBeginOverlap
  (params (OtherActor :type Actor%20Object%20Reference)))

(event EventTick
  (params (DeltaSeconds :type Float%20%28single-precision%29))
  (bind _collision (Variables|Default|Getcollision))
  (bind _returnvalue (Transformation|GetWorldLocation _collision))
  (Utilities|FlowControl|Sequence
    (:then_0
      (bind (_outhit _returnvalue_2) (Collision|SphereTraceByChannel _returnvalue (+ _returnvalue (* (Math|Vector|Normalize (Transformation|GetComponentVelocity _collision)) 5e+01)) (- (Variables|/Script/Engine.SphereComponent|GetSphereRadius (Variables|Default|Getcollision)) 1e+01) "TraceTypeQuery3" false 0 "None"))
      (if _returnvalue_2
        (bind _asbp_character_base (Utilities|Casting|CastToBP_CharacterBase (.hitactor _outhit)))
        (Default|OnHit _asbp_character_base (.hitbonename _outhit) (* (Math|Vector|Normalize (Math|Vector|MakeVector (.x (.normal _outhit)) (.y (.normal _outhit)) 0.0)) -1.0) "0, 0, 0")
        (Actor|DestroyActor)))
    (:then_1
      (Variables|Default|SetLife (- (Variables|Default|GetLife) DeltaSeconds))
      (if (< (Variables|Default|GetLife) 0.0)
        (Actor|DestroyActor)))))

(fn ConstructionScript)
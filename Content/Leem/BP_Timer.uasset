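; BP_Timer is a countdown for a timed run that starts when BP_Player overlaps its box.
; Tick uses a one-second Delay to decrement Seconds and derive Minutes, while polling BP_Finish for its Pushed flag.
; Pushing the finish records elapsed time, stops movement and shows WB_FinishRoad once.
; Reaching zero stops movement and creates WB_FailFinish every tick; timer widget, teleport, time dilation and level-load nodes are unconnected.
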(event OnComponentBeginOverlap(Box)
  (params (OverlappedComponent :type Primitive%20Component%20Object%20Reference) (OtherActor :type Actor%20Object%20Reference) (OtherComp :type Primitive%20Component%20Object%20Reference) (OtherBodyIndex :type Integer) (bFromSweep :type Boolean) (SweepResult :type Hit%20Result%20Structure%20%28by%20ref%29))
  (Utilities|Casting|CastToBP_Player OtherActor)
  (Variables|Default|SetbStart true)
  (Variables|Default|SetstartSeconds (Variables|Default|GetSeconds)))

(event EventTick
  (params (DeltaSeconds :type Float%20%28single-precision%29))
  (bind _returnvalue (Actor|GetActorOfClass "/Game/Leem/LevelObject/BP_Finish.BP_Finish_C"))
  (if (Variables|/Game/Leem/LevelObject/BP_Finish.BP_Finish_C|GetbPushed _returnvalue)
    (Variables|Default|Setrecord (- (Variables|Default|GetstartSeconds) (Variables|Default|GetSeconds)))
    (Utilities|FlowControl|DoOnce false
      (:Completed
        (Components|Movement|StopMovementImmediately (Variables|/Script/Engine.Character|GetCharacterMovement (Game|GetPlayerCharacter 0)))
        (bind _returnvalue_2 (UserInterface|CreateWidget "/Game/Leem/WB_FinishRoad.WB_FinishRoad_C"))
        (UserInterface|Viewport|AddtoViewport _returnvalue_2 0)))
    (elif (Variables|Default|GetbStart)
      (if (!= (Variables|Default|GetSeconds) 0)
        (Utilities|FlowControl|Delay 1.0)
        (bind _output_get (Variables|Default|SetSeconds (- (Variables|Default|GetSeconds) 1)))
        (Variables|Default|SetMinutes (/ _output_get 60))
        (else
          (Components|Movement|StopMovementImmediately (Variables|/Script/Engine.Character|GetCharacterMovement (Game|GetPlayerCharacter 0)))
          (bind _returnvalue_3 (UserInterface|CreateWidget "/Game/Leem/WB_FailFinish.WB_FailFinish_C"))
          (UserInterface|Viewport|AddtoViewport _returnvalue_3 0))))))

(fn ConstructionScript)
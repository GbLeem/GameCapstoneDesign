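; BP_Zone is a capture zone that fills while BP_Player stands inside its Box and prints CLEAR once captured.
; Box overlap events toggle an Overlap flag, which Tick reads to raise Point each frame or drain it toward zero.
; CheckPoint is set from a Point threshold only while overlapped, so it keeps its value during decay.
; Progress is per frame, not time-scaled, and shown only through debug prints.
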(event OnComponentBeginOverlap(Box)
  (params (OverlappedComponent :type Primitive%20Component%20Object%20Reference) (OtherActor :type Actor%20Object%20Reference) (OtherComp :type Primitive%20Component%20Object%20Reference) (OtherBodyIndex :type Integer) (bFromSweep :type Boolean) (SweepResult :type Hit%20Result%20Structure%20%28by%20ref%29))
  ;[1 1 1] 캐릭터가 zone에 들어가면 변수 set
  (Utilities|Casting|CastToBP_Player OtherActor)
  (Variables|Default|SetbOverlap true))

(event OnComponentEndOverlap(Box)
  (params (OverlappedComponent :type Primitive%20Component%20Object%20Reference) (OtherActor :type Actor%20Object%20Reference) (OtherComp :type Primitive%20Component%20Object%20Reference) (OtherBodyIndex :type Integer))
  ;[1 1 1] 캐릭터가 zone에 들어가면 변수 set
  (Utilities|Casting|CastToBP_Player OtherActor)
  (Variables|Default|SetbOverlap false))

(event EventBeginPlay)

(event EventTick
  (params (DeltaSeconds :type Float%20%28single-precision%29))
  (Utilities|FlowControl|Sequence
    (:then_0
      (if (Variables|Default|GetbOverlap)
        ;[1 1 1] 점령시 올라가는 point
        (bind _output_get (Variables|Default|Setpoint (Variables|Default|Getpoint)))
        (bind _result (Math|Integer|IncrementInt _output_get)
          (:%20%20
            ;[1 1 1] CheckPoint 변수
            (Variables|Default|SetbCheckPoint (> (Variables|Default|Getpoint) 200))
            (Development|PrintString (Utilities|String|ToString(Integer) _result))))
        (else
          (bind _output_get_2 (Variables|Default|Setpoint (Variables|Default|Getpoint)))
          (if (> _output_get_2 0)
            (bind _result_2 (Math|Integer|DecrementInt _output_get_2)
              (:%20%20
                (Development|PrintString (Utilities|String|ToString(Integer) _result_2))))))))
    (:then_1
      ;[1 1 1] 포인트 체크
      (if (Variables|Default|GetbCheckPoint)
        (Development|PrintString "CLEAR")))))

(event Collision|EventActorBeginOverlap
  (params (OtherActor :type Actor%20Object%20Reference)))

(fn ConstructionScript)
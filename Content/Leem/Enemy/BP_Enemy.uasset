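; Enemy character derived from BP_CharacterBase that starts with its own HP and constantly turns to face the player.
; Tick calls LookAtPlayer, which updates only yaw, a workaround for facing lost after reparenting.
; Throw just calls the parent, and the Hit event is empty.
; Thrown-object hit reaction, debug HP drain with low-HP random facing, and physical animation are present but disconnected, so never run.
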(event EventBeginPlay
  ;[1 1 1] enemy 체력 set
  (|CallParentFunction)
  (Variables|Default|SetEnemyHP 5e+02))

(event Collision|EventHit
  (params (MyComp :type Primitive%20Component%20Object%20Reference) (Other :type Actor%20Object%20Reference) (OtherComp :type Primitive%20Component%20Object%20Reference) (bSelfMoved :type Boolean) (HitLocation :type Vector :default "0, 0, 0") (HitNormal :type Vector :default "0, 0, 0") (NormalImpulse :type Vector :default "0, 0, 0") (Hit :type Hit%20Result%20Structure%20%28by%20ref%29))
  ;[1 1 1] 원거리 공격 받았을때
)

(event EventTick
  (params (DeltaSeconds :type Float%20%28single-precision%29))
  ;[1 1 1] BP_CharacterBase를 상속받은 이후로 enemy가 캐릭터를 바라보지 않아서 만든 함수입니다.
  (|CallParentFunction DeltaSeconds)
  (CallFunction|LookatPlayer))

(fn ConstructionScript)

(fn LookatPlayer
  (bind _returnvalue (Transformation|GetActorRotation))
  ;[1 1 1] enemy가 캐릭터를 바라보지 않아서 만든 함수입니다.
  ;[1 1 1] yaw 회전만 뽑아서 공격 후 바라보는 방향 업데이트
  (Transformation|SetActorRotation (Math|Rotator|MakeRotator (.roll _returnvalue) (.pitch _returnvalue) (.yaw (Math|Rotator|FindLookatRotation (Transformation|GetActorLocation) (Transformation|GetActorLocation (Game|GetPlayerCharacter 0)))))))

(fn NotLookatPlayer
  (if (> (Variables|Default|GetCheckTime) 5e+02)
    (Transformation|SetActorRotation (Math|Rotator|MakeRotator 0.0 0.0 (.Yaw (Math|Vector|GetYawPitchfromVector (Math|Random|RandomUnitVector)))))
    (Development|PrintString "random look")
    (Variables|Default|SetCheckTime 0.0)
    (Development|PrintString "set zero")))

(fn Throw
  (|CallParentFunction))
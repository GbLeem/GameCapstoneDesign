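; BP_EnemyController is the AI controller for enemy pawns, driving their behavior from perceived targets.
; On BeginPlay it sets up the BB_AI blackboard, runs the BT_AI behavior tree and casts the controlled pawn to BP_Enemy without using the result.
; Perception updates write any sensed actor to the BB_PlayerCharacter key, with no player filter, and clear it when sensing fails.
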(event OnTargetPerceptionUpdated(AIPerception)
  (params (Actor :type Actor%20Object%20Reference) (Stimulus :type AI%20Stimulus%20Structure))
  (bind _returnvalue (Utilities|Name|MakeLiteralName "BB_PlayerCharacter"))
  (bind _blackboard (Variables|Default|GetBlackboard))
  (if (.bSuccessfullySensed (Utilities|Struct|BreakAIStimulus Stimulus))
    (AI|Components|Blackboard|SetValueasObject _blackboard _returnvalue Actor)
    (else
      (AI|Components|Blackboard|SetValueasObject _blackboard _returnvalue 0))))

(event EventBeginPlay
  (Class|AIController|UseBlackboard "/Game/Leem/Enemy/Task/BB_AI.BB_AI")
  (AI|RunBehaviorTree "/Game/Leem/Enemy/Task/BT_AI.BT_AI")
  (Utilities|Casting|CastToBP_Enemy (Pawn|GetControlledPawn)))

(fn ConstructionScript)
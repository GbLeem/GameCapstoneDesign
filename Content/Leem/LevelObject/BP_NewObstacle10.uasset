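; Level obstacle that turns into a physics object when an actor overlaps it while the player's IsRegionActive flag is set.
; Its mesh initializes from ID in construction, then with a fixed index 5 at BeginPlay.
; StaticMesh copies the transform of the physics-driven SimulateStatic every tick.
; Parent outline functions are extended to swap a dynamic outline material onto SimulateStatic and restore the wall material on removal.
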(event EventBeginPlay
  (|CallParentFunction)
  (CallFunction|InitMesh 5))

(event Collision|EventActorBeginOverlap
  (params (OtherActor :type Actor%20Object%20Reference))
  (bind _asbp_player (Utilities|Casting|CastToBP_Player (Game|Player|GetPlayerPawn 0)))
  (if (Variables|/Game/Character/BP_Player.BP_Player_C|GetisRegionActive _asbp_player)
    (Physics|SetSimulatePhysics (Variables|Default|GetSimulateStatic) true)))

(event EventTick
  (params (DeltaSeconds :type Float%20%28single-precision%29))
  (|CallParentFunction DeltaSeconds)
  (Transformation|SetWorldTransform (Variables|Default|GetStaticMesh) (Transformation|GetWorldTransform (Variables|Default|GetSimulateStatic)) false false))

(fn ConstructionScript
  (|CallParentFunction)
  (CallFunction|InitMesh (Variables|Default|GetID)))

(fn CreateOutline
  (|CallParentFunction)
  (if (not (Variables|Default|GetHasOutline))
    (bind _returnvalue (Rendering|Material|CreateDynamicMaterialInstance (Variables|Default|GetSimulateStatic) 0 "/Game/Minjeong/SafetyRegionEffect/Outline/M_Outline_Inst.M_Outline_Inst" "None" :!class /Script/Engine.PrimitiveComponent))
    (bind _output_get (Variables|Default|SetDMI _returnvalue))
    (Rendering|Material|SetScalarParameterValue _output_get "Scale" 3.0 :!class /Script/Engine.MaterialInstanceDynamic)
    (Variables|Default|SetHasOutline true)))

(fn DeleteOutline
  (bind _dmi (Variables|Default|GetDMI))
  (|CallParentFunction)
  (if (Variables|Default|GetHasOutline)
    (Rendering|Material|SetScalarParameterValue _dmi "scale" 0.0 :!class /Script/Engine.MaterialInstanceDynamic)
    (Rendering|Material|SetVectorParameterValue _dmi "color" (Utilities|Struct|MakeLinearColor 0.0 0.0 0.0 0.0) :!class /Script/Engine.MaterialInstanceDynamic)
    (Rendering|Material|SetMaterial (Variables|Default|GetSimulateStatic) 0 "/Game/FunObstacleCourse/Mesh/Materials/MI_Wall_1.MI_Wall_1")
    (Variables|Default|SetHasOutline false)))
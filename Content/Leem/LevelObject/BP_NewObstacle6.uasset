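; Level obstacle that sets up its mesh through InitMesh and knocks the player when touched.
; Overlapping SimulateStatic turns off the player's physical animation if a region is active; otherwise it activates it and, after a short delay, applies an impulse below the anchor bone.
; Tick snaps static meshes to SimulateStatic's transform.
; Outline overrides swap SimulateStatic's material between a dynamic outline instance and the ball material.
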(event OnComponentBeginOverlap(SimulateStatic)
  (params (OverlappedComponent :type Primitive%20Component%20Object%20Reference) (OtherActor :type Actor%20Object%20Reference) (OtherComp :type Primitive%20Component%20Object%20Reference) (OtherBodyIndex :type Integer) (bFromSweep :type Boolean) (SweepResult :type Hit%20Result%20Structure%20%28by%20ref%29))
  (bind _asbp_player (Utilities|Casting|CastToBP_Player OtherActor))
  (if (Variables|/Game/Character/BP_Player.BP_Player_C|GetisRegionActive _asbp_player)
    (Default|DeactivatePhysicalAnimation _asbp_player)
    (else
      (Default|ActivatePhysicalAnimation _asbp_player 0.25)
      (Utilities|FlowControl|Delay 0.2)
      (Class|SkeletalMeshComponent|AddImpulsetoAllBodiesBelow (Variables|/Script/Engine.Character|GetMesh _asbp_player) "100.000000,100.000000,300.000000" (Variables|/Game/Character/BP_CharacterBase.BP_CharacterBase_C|GetAnchorBone _asbp_player) false true))))

(event EventBeginPlay
  (|CallParentFunction)
  (CallFunction|InitMesh 4))

(event Collision|EventActorBeginOverlap
  (params (OtherActor :type Actor%20Object%20Reference)))

(event EventTick
  (params (DeltaSeconds :type Float%20%28single-precision%29))
  (|CallParentFunction DeltaSeconds)
  (Transformation|SetWorldTransform (Variables|Default|GetStaticMesh) (Transformation|GetWorldTransform (Variables|Default|GetSimulateStatic)) false false))

(fn ConstructionScript
  (|CallParentFunction)
  (CallFunction|InitMesh (Variables|Default|GetID)))

(fn CreateOutline
  (|CallParentFunction)
  (if (not (Variables|Default|GetHasOutline))
    (bind _returnvalue (Rendering|Material|CreateDynamicMaterialInstance (Variables|Default|GetSimulateStatic) 0 "/Game/Minjeong/SafetyRegionEffect/Outline/M_Outline_Inst.M_Outline_Inst" "None" :!class /Script/Engine.PrimitiveComponent))
    (bind _output_get (Variables|Default|SetDMI_0 _returnvalue))
    (Rendering|Material|SetScalarParameterValue _output_get "Scale" 3.0 :!class /Script/Engine.MaterialInstanceDynamic)
    (Variables|Default|SetHasOutline true)))

(fn DeleteOutline
  (bind _dmi_0 (Variables|Default|GetDMI_0))
  (|CallParentFunction)
  (if (Variables|Default|GetHasOutline)
    (Rendering|Material|SetScalarParameterValue _dmi_0 "scale" 0.0 :!class /Script/Engine.MaterialInstanceDynamic)
    (Rendering|Material|SetVectorParameterValue _dmi_0 "color" (Utilities|Struct|MakeLinearColor 0.0 0.0 0.0 0.0) :!class /Script/Engine.MaterialInstanceDynamic)
    (Rendering|Material|SetMaterial (Variables|Default|GetSimulateStatic) 0 "/Game/FunObstacleCourse/Mesh/Materials/MI_Ball_1.MI_Ball_1")
    (Variables|Default|SetHasOutline false)))
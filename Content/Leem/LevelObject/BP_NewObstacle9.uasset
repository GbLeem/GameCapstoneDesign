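; BP_NewObstacle9 is a launcher obstacle that repeatedly fires BP_NewObstacle6 actors.
; A two-second Delay on Tick paces the shots, each spawned at the Arrow component's transform with a short lifespan.
; Each projectile's SimulateStatic component receives a physics velocity pointing from the launcher's origin toward the spawn point, so the Arrow's offset sets the firing direction.
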(event EventBeginPlay)

(event Collision|EventActorBeginOverlap
  (params (OtherActor :type Actor%20Object%20Reference)))

(event EventTick
  (params (DeltaSeconds :type Float%20%28single-precision%29))
  (Utilities|FlowControl|Delay 2.0)
  (bind _returnvalue (Game|SpawnActorfromClass "/Game/Leem/LevelObject/BP_NewObstacle6.BP_NewObstacle6_C" (Math|Transform|MakeTransform (Transformation|GetWorldLocation (Variables|Default|GetArrow)) (Transformation|GetWorldRotation (Variables|Default|GetArrow)) "1.000000,1.000000,1.000000") "Undefined" 0 0))
  (Actor|SetLifeSpan _returnvalue 1.5)
  (Physics|SetPhysicsLinearVelocity (Variables|/Game/Minjeong/Actor/BP_NewParentObstacle.BP_NewParentObstacle_C|GetSimulateStatic _returnvalue) (* (Math|Vector|GetUnitDirection(Vector) (Transformation|GetActorLocation) (Transformation|GetActorLocation _returnvalue)) 1e+03) false "None"))

(fn ConstructionScript)
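; BP_NewObstacle8 is a level obstacle that swings its Base component back and forth in pitch.
; Two timelines drive the rotation, one played from start and the other reversed from end.
; Each timeline's Update runs through a three-second Delay that starts the other timeline, forming a repeating cycle from BeginPlay.
; Overlap of the One component with BP_Player only prints a debug "hit" message.
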(event OnComponentBeginOverlap(one)
  (params (OverlappedComponent :type Primitive%20Component%20Object%20Reference) (OtherActor :type Actor%20Object%20Reference) (OtherComp :type Primitive%20Component%20Object%20Reference) (OtherBodyIndex :type Integer) (bFromSweep :type Boolean) (SweepResult :type Hit%20Result%20Structure%20%28by%20ref%29))
  (Utilities|Casting|CastToBP_Player OtherActor)
  (Development|PrintString "hit"))

(event EventBeginPlay
  (bind _새_트랙_0 (Timeline|타임라인_0 PlayFromStart)
    (:Update
      (Transformation|SetRelativeRotation (Variables|Default|Getbase) (Math|Rotator|MakeRotator 0.0 _새_트랙_0 0.0) false false)
      (Utilities|FlowControl|Delay 3.0)
      (bind _새_트랙_0_2 (Timeline|타임라인_1 ReverseFromEnd)
        (:Update
          (Transformation|SetRelativeRotation (Variables|Default|Getbase) (Math|Rotator|MakeRotator 0.0 _새_트랙_0_2 0.0) false false)
          (Utilities|FlowControl|Delay 3.0)
          (Timeline|타임라인_0 PlayFromStart))))))

(fn ConstructionScript)
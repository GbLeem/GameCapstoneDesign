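; BP_NewObstacle7 is a level obstacle that can toggle an outline highlight and initializes its mesh from an ID during construction.
; Every tick, it copies the world transform of SimulateStatic onto SimulateStatic1, keeping the second component aligned with the first.
; CreateOutline applies a dynamic outline material to SimulateStatic, and DeleteOutline restores the solid blue material, both extending parent logic and guarded by HasOutline.
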(event EventBeginPlay
  (|CallParentFunction) ; 지금 이 노드는 비활성 상태입니다. \n핀을 끌어서 다른 노드를 연결하면 활성화됩니다.
)

(event Collision|EventActorBeginOverlap
  (params (OtherActor :type Actor%20Object%20Reference)))

(event EventTick
  (params (DeltaSeconds :type Float%20%28single-precision%29))
  (|CallParentFunction DeltaSeconds)
  (Transformation|SetWorldTransform (Variables|Default|GetSimulateStatic1) (Transformation|GetWorldTransform (Variables|Default|GetSimulateStatic)) false false))

(fn ConstructionScript
  (|CallParentFunction)
  (CallFunction|InitMesh (Variables|Default|GetID)))

(fn CreateOutline
  (|CallParentFunction)
  (if (not (Variables|Default|GetHasOutline))
    (bind _returnvalue (Rendering|Material|CreateDynamicMaterialInstance (Variables|Default|GetSimulateStatic) 0 "/Game/Minjeong/SafetyRegionEffect/Outline/M_Outline_Inst.M_Outline_Inst" "None" :!class /Script/Engine.PrimitiveComponent))
    (bind _output_get (Variables|Default|SetDMI _returnvalue))
    (Rendering|Material|SetScalarParameterValue _output_get "Scale" 2.0 :!class /Script/Engine.MaterialInstanceDynamic)
    (Variables|Default|SetHasOutline true)))

(fn DeleteOutline
  (bind _dmi (Variables|Default|GetDMI))
  (|CallParentFunction)
  (if (Variables|Default|GetHasOutline)
    (Rendering|Material|SetScalarParameterValue _dmi "scale" 0.0 :!class /Script/Engine.MaterialInstanceDynamic)
    (Rendering|Material|SetVectorParameterValue _dmi "color" (Utilities|Struct|MakeLinearColor 0.0 0.0 0.0 0.0) :!class /Script/Engine.MaterialInstanceDynamic)
    (Rendering|Material|SetMaterial (Variables|Default|GetSimulateStatic) 0 "/Game/LevelPrototyping/Materials/MI_Solid_Blue.MI_Solid_Blue")
    (Variables|Default|SetHasOutline false)))
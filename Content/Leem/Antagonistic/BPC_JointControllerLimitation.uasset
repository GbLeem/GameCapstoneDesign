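; Joint controller component that computes an antagonistic torque from a joint's orientation relative to its angular limits.
; Per axis, it extracts the twist rotation and measures the signed angle's error to the soft min and max limits.
; Three internal antagonistic gain controllers turn these errors into torque, which is then scaled using the body's inertia tensor.
; Kinematic errors and gravity torque do not affect the output, and the velocity term is zero.
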(event EventBeginPlay)

(event EventTick
  (params (DeltaSeconds :type Float%20%28single-precision%29)))

(fn Constructor
  (params (plx :type Float%20%28double-precision%29) (phx :type Float%20%28double-precision%29) (kix :type Float%20%28double-precision%29) (kdx :type Float%20%28double-precision%29) (ply :type Float%20%28double-precision%29) (phy :type Float%20%28double-precision%29) (kiy :type Float%20%28double-precision%29) (kdy :type Float%20%28double-precision%29) (plz :type Float%20%28double-precision%29) (phz :type Float%20%28double-precision%29) (kiz :type Float%20%28double-precision%29) (kdz :type Float%20%28double-precision%29))
  (bind __internalantagonisticcontroller (Variables|Default|Get_internalAntagonisticController))
  (if (Math|Boolean|ORBoolean (< plx 0.0) (< phx 0.0) (< kix 0.0) (< kdx 0.0) (< ply 0.0) (< phy 0.0) (< kiy 0.0) (< kdy 0.0) (< plz 0.0) (< phz 0.0) (< kiz 0.0) (< kdz 0.0))
    (Development|PrintString "throw exception")
    (else
      (Default|Constructor __internalantagonisticcontroller plx phx kix kdx)
      (Default|Constructor __internalantagonisticcontroller ply phy kiy kdy)
      (Default|Constructor __internalantagonisticcontroller plz phz kiz kdz))))

(fn KPLX
  (return (Variables|/Game/Leem/Antagonistic/BPC_AntagonisticController.BPC_AntagonisticController_C|Get_kPL (Utilities|Array|Get(acopy) (Variables|Default|Get_internalAntagonisticController)))))

(fn KPHX
  (return (Variables|/Game/Leem/Antagonistic/BPC_AntagonisticController.BPC_AntagonisticController_C|Get_kPH (Utilities|Array|Get(acopy) (Variables|Default|Get_internalAntagonisticController)))))

(fn KDX
  (return (Variables|/Game/Leem/Antagonistic/BPC_AntagonisticController.BPC_AntagonisticController_C|Get_kD (Utilities|Array|Get(acopy) (Variables|Default|Get_internalAntagonisticController)))))

(fn KIX
  (return (Variables|/Game/Leem/Antagonistic/BPC_AntagonisticController.BPC_AntagonisticController_C|Get_kI (Utilities|Array|Get(acopy) (Variables|Default|Get_internalAntagonisticController)))))

(fn KPLY
  (return (Variables|/Game/Leem/Antagonistic/BPC_AntagonisticController.BPC_AntagonisticController_C|Get_kPL (Utilities|Array|Get(acopy) (Variables|Default|Get_internalAntagonisticController) 1))))

(fn KPHY
  (return (Variables|/Game/Leem/Antagonistic/BPC_AntagonisticController.BPC_AntagonisticController_C|Get_kPH (Utilities|Array|Get(acopy) (Variables|Default|Get_internalAntagonisticController) 1))))

(fn KDY
  (return (Variables|/Game/Leem/Antagonistic/BPC_AntagonisticController.BPC_AntagonisticController_C|Get_kD (Utilities|Array|Get(acopy) (Variables|Default|Get_internalAntagonisticController) 1))))

(fn KIY
  (return (Variables|/Game/Leem/Antagonistic/BPC_AntagonisticController.BPC_AntagonisticController_C|Get_kI (Utilities|Array|Get(acopy) (Variables|Default|Get_internalAntagonisticController) 1))))

(fn KPLZ
  (return (Variables|/Game/Leem/Antagonistic/BPC_AntagonisticController.BPC_AntagonisticController_C|Get_kPL (Utilities|Array|Get(acopy) (Variables|Default|Get_internalAntagonisticController) 2))))

(fn KPHZ
  (return (Variables|/Game/Leem/Antagonistic/BPC_AntagonisticController.BPC_AntagonisticController_C|Get_kPH (Utilities|Array|Get(acopy) (Variables|Default|Get_internalAntagonisticController) 2))))

(fn KDZ
  (return (Variables|/Game/Leem/Antagonistic/BPC_AntagonisticController.BPC_AntagonisticController_C|Get_kD (Utilities|Array|Get(acopy) (Variables|Default|Get_internalAntagonisticController) 2))))

(fn KIZ
  (return (Variables|/Game/Leem/Antagonistic/BPC_AntagonisticController.BPC_AntagonisticController_C|Get_kI (Utilities|Array|Get(acopy) (Variables|Default|Get_internalAntagonisticController) 2))))

(fn ComputeRequiredAntagonisticTorque
  (params (minSoftLimitX :type Float%20%28double-precision%29) (maxSoftLimitX :type Float%20%28double-precision%29) (minSoftLimitY :type Float%20%28double-precision%29) (maxSoftLimitY :type Float%20%28double-precision%29) (minSoftLimitZ :type Float%20%28double-precision%29) (maxSoftLimitZ :type Float%20%28double-precision%29) (minHardLimitX :type Float%20%28double-precision%29) (maxHardLimitX :type Float%20%28double-precision%29) (minHardLimitY :type Float%20%28double-precision%29) (maxHardLimitY :type Float%20%28double-precision%29) (minHardLimitZ :type Float%20%28double-precision%29) (maxHardLimitZ :type Float%20%28double-precision%29) (currentTransform :type Transform) (currentLocalOrientation :type Quat%20Structure) (kinematicLocalOrientation :type Quat%20Structure) (_objectRigidbody :type Primitive%20Component%20Object%20Reference) (gravityTorqueLocal :type Vector) (fixedDeltaTime :type Float%20%28double-precision%29) (gameobject :type Actor%20Object%20Reference))
  (bind _returnvalue (Class|PrimitiveComponent|GetInertiaTensor _objectRigidbody "None"))
  (Utilities|FlowControl|Sequence
    (:then_0
      ;[1 1 1] region Orientations - X
      (bind _twistreturn (CallFunction|GetRotationComponentAboutAxis currentLocalOrientation "1.000000, 0, 0"))
      (LocalVariables|SetcurrentLocalOrientationQuaternionX _twistreturn)
      (bind _twistreturn_2 (CallFunction|GetRotationComponentAboutAxis kinematicLocalOrientation "1.000000, 0, 0"))
      (LocalVariables|SetkinematicLocalOrientationQuaternionX _twistreturn_2)
      (LocalVariables|SetcurrentLocalOrientationQuaternionXAngle (Class|KismetMathLibrary|QuatGetAngle (LocalVariables|GetcurrentLocalOrientationQuaternionX)))
      (LocalVariables|SetcurrentLocalOrientationQuaternionXAxis (Class|KismetMathLibrary|QuatGetRotationAxis (LocalVariables|GetcurrentLocalOrientationQuaternionX)))
      (Class|KismetMathLibrary|QuatNormalize (LocalVariables|GetcurrentLocalOrientationQuaternionX) 0.0001)
      (LocalVariables|SetkinematicLocalOrientationQuaternionXAngle (Class|KismetMathLibrary|QuatGetAngle (LocalVariables|GetkinematicLocalOrientationQuaternionX)))
      (LocalVariables|SetkinematicLocalOrientationQuaternionXAxis (Class|KismetMathLibrary|QuatGetRotationAxis (LocalVariables|GetkinematicLocalOrientationQuaternionX)))
      (Class|KismetMathLibrary|QuatNormalize (LocalVariables|GetkinematicLocalOrientationQuaternionX) 0.0001)
      (Utilities|FlowControl|Sequence
        (:then_0
          (if (> (LocalVariables|GetcurrentLocalOrientationQuaternionXAngle) 1.8e+02)
            (LocalVariables|SetcurrentLocalOrientationQuaternionXAngleCorrected (- (LocalVariables|GetcurrentLocalOrientationQuaternionXAngle) 3.6e+02))
            (else
              (LocalVariables|SetcurrentLocalOrientationQuaternionXAngleCorrected (LocalVariables|GetcurrentLocalOrientationQuaternionXAngle)))))
        (:then_1
          (if (> (LocalVariables|GetkinematicLocalOrientationQuaternionXAngle) 1.8e+02)
            (LocalVariables|SetkinematicLocalOrientationQuaternionXAngleCorrected (- (LocalVariables|GetkinematicLocalOrientationQuaternionXAngle) 3.6e+02))
            (else
              (LocalVariables|SetkinematicLocalOrientationQuaternionXAngleCorrected (LocalVariables|GetkinematicLocalOrientationQuaternionXAngle)))))
        (:then_2
          ;[1 1 1] Estimate Errors directly from Axis-Angle - X
          (LocalVariables|SetcurrentLocalErrorMinX (- minSoftLimitX (LocalVariables|GetcurrentLocalOrientationQuaternionXAngleCorrected)))
          (LocalVariables|SetcurrentLocalErrorMaxX (- maxSoftLimitX (LocalVariables|GetcurrentLocalOrientationQuaternionXAngleCorrected)))
          (LocalVariables|SetkinematicLocalErrorMinX (- minSoftLimitX (LocalVariables|GetkinematicLocalOrientationQuaternionXAngleCorrected)))
          (LocalVariables|SetkinematicLocalErrorMaxX (- maxSoftLimitX (LocalVariables|GetkinematicLocalOrientationQuaternionXAngleCorrected)))
          (LocalVariables|SetkinematicLocalErrorMinXClamp (Math|Float|Clamp(Float) (LocalVariables|GetkinematicLocalErrorMinX) (- minSoftLimitX maxHardLimitX) (- minSoftLimitX minHardLimitX)))
          (LocalVariables|SetkinematicLocalErrorMaxXClamp (Math|Float|Clamp(Float) (LocalVariables|GetkinematicLocalErrorMaxX) (- maxSoftLimitX maxHardLimitX) (- maxSoftLimitX minHardLimitX))))))
    (:then_1
      ;[1 1 1] region Orientations - Y
      (bind _twistreturn_3 (CallFunction|GetRotationComponentAboutAxis currentLocalOrientation "0.000000,1.000000, 0"))
      (LocalVariables|SetcurrentLocalOrientationQuaternionY _twistreturn_3)
      (bind _twistreturn_4 (CallFunction|GetRotationComponentAboutAxis kinematicLocalOrientation "0.000000,1.000000, 0"))
      (LocalVariables|SetkinematicLocalOrientationQuaternionY _twistreturn_4)
      (LocalVariables|SetcurrentLocalOrientationQuaternionYAngle (Class|KismetMathLibrary|QuatGetAngle (LocalVariables|GetcurrentLocalOrientationQuaternionY)))
      (LocalVariables|SetcurrentLocalOrientationQuaternionYAxis (Class|KismetMathLibrary|QuatGetRotationAxis (LocalVariables|GetcurrentLocalOrientationQuaternionY)))
      (Class|KismetMathLibrary|QuatNormalize (LocalVariables|GetcurrentLocalOrientationQuaternionY) 0.0001)
      (LocalVariables|SetkinematicLocalOrientationQuaternionYAngle (Class|KismetMathLibrary|QuatGetAngle (LocalVariables|GetkinematicLocalOrientationQuaternionY)))
      (LocalVariables|SetkinematicLocalOrientationQuaternionYAxis (Class|KismetMathLibrary|QuatGetRotationAxis (LocalVariables|GetkinematicLocalOrientationQuaternionY)))
      (Class|KismetMathLibrary|QuatNormalize (LocalVariables|GetkinematicLocalOrientationQuaternionY) 0.0001)
      (Utilities|FlowControl|Sequence
        (:then_0
          (if (> (LocalVariables|GetcurrentLocalOrientationQuaternionYAngle) 1.8e+02)
            (LocalVariables|SetcurrentLocalOrientationQuaternionYAngleCorrected (- (LocalVariables|GetcurrentLocalOrientationQuaternionYAngle) 3.6e+02))
            (else
              (LocalVariables|SetcurrentLocalOrientationQuaternionYAngleCorrected (LocalVariables|GetcurrentLocalOrientationQuaternionYAngle)))))
        (:then_1
          (if (> (LocalVariables|GetkinematicLocalOrientationQuaternionYAngle) 1.8e+02)
            (LocalVariables|SetkinematicLocalOrientationQuaternionYAngleCorrected (- (LocalVariables|GetkinematicLocalOrientationQuaternionYAngle) 3.6e+02))
            (else
              (LocalVariables|SetkinematicLocalOrientationQuaternionYAngleCorrected (LocalVariables|GetkinematicLocalOrientationQuaternionYAngle)))))
        (:then_2
          ;[1 1 1] Estimate Errors directly from Axis-Angle - Y
          (LocalVariables|SetcurrentLocalErrorMinY (- minSoftLimitY (LocalVariables|GetcurrentLocalOrientationQuaternionYAngleCorrected)))
          (LocalVariables|SetcurrentLocalErrorMaxY (- maxSoftLimitY (LocalVariables|GetcurrentLocalOrientationQuaternionYAngleCorrected)))
          (LocalVariables|SetkinematicLocalErrorMinY (- minSoftLimitY (LocalVariables|GetkinematicLocalOrientationQuaternionYAngleCorrected)))
          (LocalVariables|SetkinematicLocalErrorMaxY (- maxSoftLimitY (LocalVariables|GetkinematicLocalOrientationQuaternionYAngleCorrected)))
          (LocalVariables|SetkinematicLocalErrorMinYClamp (Math|Float|Clamp(Float) (LocalVariables|GetkinematicLocalErrorMinY) (- minSoftLimitY maxHardLimitY) (- minSoftLimitY minHardLimitY)))
          (LocalVariables|SetkinematicLocalErrorMaxYClamp (Math|Float|Clamp(Float) (LocalVariables|GetkinematicLocalErrorMaxY) (- maxSoftLimitY maxHardLimitY) (- maxSoftLimitY minHardLimitY))))))
    (:then_2
      ;[1 1 1] region Orientations - Z
      (bind _twistreturn_5 (CallFunction|GetRotationComponentAboutAxis currentLocalOrientation "0.000000,0.000000,1.000000"))
      (LocalVariables|SetcurrentLocalOrientationQuaternionZ _twistreturn_5)
      (bind _twistreturn_6 (CallFunction|GetRotationComponentAboutAxis kinematicLocalOrientation "0.000000,0.000000,1.000000"))
      (LocalVariables|SetkinematicLocalOrientationQuaternionZ _twistreturn_6)
      (LocalVariables|SetcurrentLocalOrientationQuaternionZAngle (Class|KismetMathLibrary|QuatGetAngle (LocalVariables|GetcurrentLocalOrientationQuaternionZ)))
      (LocalVariables|SetcurrentLocalOrientationQuaternionZAxis (Class|KismetMathLibrary|QuatGetRotationAxis (LocalVariables|GetcurrentLocalOrientationQuaternionZ)))
      (Class|KismetMathLibrary|QuatNormalize (LocalVariables|GetcurrentLocalOrientationQuaternionZ) 0.0001)
      (LocalVariables|SetkinematicLocalOrientationQuaternionZAngle (Class|KismetMathLibrary|QuatGetAngle (LocalVariables|GetkinematicLocalOrientationQuaternionZ)))
      (LocalVariables|SetkinematicLocalOrientationQuaternionZAxis (Class|KismetMathLibrary|QuatGetRotationAxis (LocalVariables|GetkinematicLocalOrientationQuaternionZ)))
      (Class|KismetMathLibrary|QuatNormalize (LocalVariables|GetkinematicLocalOrientationQuaternionZ) 0.0001)
      (Utilities|FlowControl|Sequence
        (:then_0
          (if (> (LocalVariables|GetcurrentLocalOrientationQuaternionZAngle) 1.8e+02)
            (LocalVariables|SetcurrentLocalOrientationQuaternionZAngleCorrected (- (LocalVariables|GetcurrentLocalOrientationQuaternionZAngle) 3.6e+02))
            (else
              (LocalVariables|SetcurrentLocalOrientationQuaternionZAngleCorrected (LocalVariables|GetcurrentLocalOrientationQuaternionZAngle)))))
        (:then_1
          (if (> (LocalVariables|GetkinematicLocalOrientationQuaternionZAngle) 1.8e+02)
            (LocalVariables|SetkinematicLocalOrientationQuaternionZAngleCorrected (- (LocalVariables|GetkinematicLocalOrientationQuaternionZAngle) 3.6e+02))
            (else
              (LocalVariables|SetkinematicLocalOrientationQuaternionZAngleCorrected (LocalVariables|GetkinematicLocalOrientationQuaternionZAngle)))))
        (:then_2
          ;[1 1 1] Estimate Errors directly from Axis-Angle - Z
          (LocalVariables|SetcurrentLocalErrorMinZ (- minSoftLimitZ (LocalVariables|GetcurrentLocalOrientationQuaternionZAngleCorrected)))
          (LocalVariables|SetcurrentLocalErrorMaxZ (- maxSoftLimitZ (LocalVariables|GetcurrentLocalOrientationQuaternionZAngleCorrected)))
          (LocalVariables|SetkinematicLocalErrorMinZ (- minSoftLimitZ (LocalVariables|GetkinematicLocalOrientationQuaternionZAngleCorrected)))
          (LocalVariables|SetkinematicLocalErrorMinZ (- maxSoftLimitZ (LocalVariables|GetkinematicLocalOrientationQuaternionZAngleCorrected)))
          (LocalVariables|SetkinematicLocalErrorMinZClamp (Math|Float|Clamp(Float) (LocalVariables|GetkinematicLocalErrorMinZ) (- minSoftLimitZ maxHardLimitZ) (- minSoftLimitZ minHardLimitZ)))
          (LocalVariables|SetkinematicLocalErrorMinZClamp (Math|Float|Clamp(Float) (LocalVariables|GetkinematicLocalErrorMaxZ) (- maxSoftLimitZ maxHardLimitZ) (- maxSoftLimitZ minHardLimitZ))))))
    (:then_3
      ;[1 1 1] torque estimation
      (bind _outputreturn (CallFunction|GetOutput (LocalVariables|GetcurrentLocalErrorMinX) (LocalVariables|GetcurrentLocalErrorMaxX) (LocalVariables|GetcurrentLocalErrorMinY) (LocalVariables|GetcurrentLocalErrorMaxY) (LocalVariables|GetcurrentLocalErrorMinZ) (LocalVariables|GetcurrentLocalErrorMaxZ) (Math|Vector|VectorLength "0, 0, 0") fixedDeltaTime))
      (LocalVariables|SettorqueApplied _outputreturn)
      ;[1 1 1] Intertia
      (LocalVariables|SettorqueApplied (* (Class|KismetMathLibrary|QuatGetRotationAxis (Math|Conversions|ToQuaternion(Rotator) (Class|PrimitiveComponent|GetInertiaTensor _objectRigidbody "None"))) (LocalVariables|GettorqueApplied)))
      (LocalVariables|SettorqueApplied (Math|Vector|MakeVector (* (.x (LocalVariables|GettorqueApplied)) (.x _returnvalue)) (* (.y (LocalVariables|GettorqueApplied)) (.y _returnvalue)) (* (.z (LocalVariables|GettorqueApplied)) (.z _returnvalue))))
      (LocalVariables|SettorqueApplied (* (Class|KismetMathLibrary|QuatGetRotationAxis (Class|KismetMathLibrary|QuatInversed (Math|Conversions|ToQuaternion(Rotator) (Class|PrimitiveComponent|GetInertiaTensor _objectRigidbody "None")))) (LocalVariables|GettorqueApplied))))
    (:then_4
      ;[1 1 1] Return
      (return (LocalVariables|GettorqueApplied)))))

(fn GetRotationComponentAboutAxis
  (params (rotation :type Quat%20Structure) (direction :type Vector))
  (LocalVariables|SetrotattionAxis (Math|Vector|MakeVector (.x rotation) (.y rotation) (.z rotation)))
  (LocalVariables|SetdotProd (Math|Vector|DotProduct (LocalVariables|GetrotattionAxis) direction))
  (LocalVariables|Setprojection (Math|Vector|MakeVector (* (.x rotation) (LocalVariables|GetdotProd)) (* (.y rotation) (LocalVariables|GetdotProd)) (* (.z rotation) (LocalVariables|GetdotProd))))
  (bind _output_get (LocalVariables|Settwist (Class|KismetMathLibrary|MakeQuat (.x (LocalVariables|Getprojection)) (.y (LocalVariables|Getprojection)) (.z (LocalVariables|Getprojection)) (.w rotation))))
  (Class|KismetMathLibrary|QuatNormalize _output_get 0.0001)
  (if (< (LocalVariables|GetdotProd) 0.0)
    (LocalVariables|Settwist (Utilities|Struct|MakeQuat (* (.x (LocalVariables|Gettwist)) -1.0) (* (.y (LocalVariables|Gettwist)) -1.0) (* (.z (LocalVariables|Gettwist)) -1.0) (* (.w (LocalVariables|Gettwist)) -1.0))))
  (return (LocalVariables|Gettwist)))

(fn GetOutput
  (params (lowErrorX :type Float%20%28double-precision%29) (highErrorX :type Float%20%28double-precision%29) (lowErrorY :type Float%20%28double-precision%29) (highErrorY :type Float%20%28double-precision%29) (lowErrorZ :type Float%20%28double-precision%29) (highErrorZ :type Float%20%28double-precision%29) (delta :type Float%20%28double-precision%29) (deltaTime :type Float%20%28double-precision%29))
  (bind _antagonisticreturn (Default|GetOuput (Utilities|Array|Get(acopy) (Variables|Default|Get_internalAntagonisticController)) lowErrorX highErrorX delta deltaTime))
  (bind _antagonisticreturn_2 (Default|GetOuput (Utilities|Array|Get(acopy) (Variables|Default|Get_internalAntagonisticController) 1) lowErrorY highErrorY delta deltaTime))
  (bind _antagonisticreturn_3 (Default|GetOuput (Utilities|Array|Get(acopy) (Variables|Default|Get_internalAntagonisticController) 2) lowErrorZ highErrorZ delta deltaTime))
  (bind _output_get (LocalVariables|Setoutput (Math|Vector|MakeVector _antagonisticreturn _antagonisticreturn_2 _antagonisticreturn_3)))
  (return _output_get))
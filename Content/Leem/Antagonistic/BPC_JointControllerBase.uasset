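; BPC_JointControllerBase is a work-in-progress joint controller component for antagonistic PD control of a limb.
; BeginPlay stores the kinematic limb's transform and clears the current transform and rigid body references.
; Tick sets the XYZ controller to None, calls its Constructor with per-axis gains, then queries its gain functions, though the Y derivative step calls KDX again.
; Disconnected chains prototype reading and setting hand constraint angular limits and looking up player physics bodies.
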(event EventBeginPlay
  ;[1 1 1] Awake
  (Variables|Read-only&StaticField|Set_currentTransform "")
  (Variables|Read-only&StaticField|Set_kinematicTransform (Transformation|GetActorTransform (Variables|GeneralSettings|GetkinematicLimb)))
  (Variables|Read-only&StaticField|Set_objectRIgidbody 0))

(event EventTick
  (params (DeltaSeconds :type Float%20%28single-precision%29))
  (Utilities|FlowControl|Sequence
    (:then_2
      (bind _output_get (Variables|Read-only&StaticField|Set_antagonisticControllerXYZ 0))
      (Default|Constructor _output_get 1.0 0.0 0.0 0.01 1.0 0.0 0.0 0.01 1.0 0.0 0.0 0.01)
      ;[1 1 1] antagonistic PD controller with middle array -415
      (Utilities|FlowControl|Sequence
        (:then_0
          (Default|KPLX (Variables|Read-only&StaticField|Get_antagonisticControllerXYZ))
          (Variables|Default|SetKPLXreturn (Variables|AntagonisticController-Settings-X|GetpLX)))
        (:then_1
          (Default|KIX (Variables|Read-only&StaticField|Get_antagonisticControllerXYZ))
          (Variables|Default|SetKIXreturn (Variables|AntagonisticController-Settings-X|GetiX)))
        (:then_2
          (Default|KDX (Variables|Read-only&StaticField|Get_antagonisticControllerXYZ))
          (Variables|Default|SetKDXreturn (Variables|AntagonisticController-Settings-X|GetdX)))
        (:then_3
          (Default|KPLY (Variables|Read-only&StaticField|Get_antagonisticControllerXYZ)))
        (:then_4
          (Default|KIY (Variables|Read-only&StaticField|Get_antagonisticControllerXYZ)))
        (:then_5
          (Default|KDX (Variables|Read-only&StaticField|Get_antagonisticControllerXYZ)))
        (:then_6
          (Default|KPLZ (Variables|Read-only&StaticField|Get_antagonisticControllerXYZ)))
        (:then_7
          (Default|KIZ (Variables|Read-only&StaticField|Get_antagonisticControllerXYZ)))
        (:then_8
          (Default|KDZ (Variables|Read-only&StaticField|Get_antagonisticControllerXYZ)))))
    (:then_3
      ;[1 1 1] 429
      (Utilities|FlowControl|Sequence
        (:then_0
          (bind _kphxreturn (Default|KPHX (Variables|Read-only&StaticField|Get_antagonisticControllerXYZ)))
          (Variables|AntagonisticController-Settings-X|SetpHX _kphxreturn))
        (:then_1
          (bind _kphyreturn (Default|KPHY (Variables|Read-only&StaticField|Get_antagonisticControllerXYZ)))
          (Variables|AntagonisticController-Settings-Y|SetpHY _kphyreturn))
        (:then_2
          (bind _kphzreturn (Default|KPHZ (Variables|Read-only&StaticField|Get_antagonisticControllerXYZ)))
          (Variables|AntagonisticController-Settings-Z|SetpHZ _kphzreturn))))))
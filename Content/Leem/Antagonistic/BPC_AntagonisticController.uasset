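; BPC_AntagonisticController is a component that computes a PID-style control output with separate low and high proportional terms.
; Constructor stores the four gains, and BeginPlay calls it without passing values.
; GetOuput returns the weighted sum of low error, high error, the supplied delta and an integral term.
; The integral term is only the current low error times Dt, with no accumulation between calls.
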(event EventBeginPlay
  (CallFunction|Constructor 0.0 0.0 0.0 0.0))

(fn Constructor
  (params (pL :type Float%20%28double-precision%29) (pH :type Float%20%28double-precision%29) (i :type Float%20%28double-precision%29) (d :type Float%20%28double-precision%29))
  (Variables|InstanceFiled|Set_kPL pL)
  (Variables|InstanceFiled|Set_kPH pH)
  (Variables|InstanceFiled|Set_kI i)
  (Variables|InstanceFiled|Set_kD d))

(fn GetOuput
  (params (CurrentLowError :type Float%20%28double-precision%29) (CurrentHighError :type Float%20%28double-precision%29) (Delta :type Float%20%28double-precision%29) (Dt :type Float%20%28double-precision%29))
  (bind _output_get (Variables|InstanceFiled|Set_PL CurrentLowError))
  (bind _output_get_2 (Variables|InstanceFiled|Set_PH CurrentHighError))
  (Variables|InstanceFiled|Set_P CurrentLowError)
  (bind _output_get_3 (Variables|InstanceFiled|Set_D Delta))
  (bind _output_get_4 (Variables|InstanceFiled|Set_I (* Dt (Variables|InstanceFiled|Get_P))))
  (return (+ (* _output_get (Variables|InstanceFiled|Get_kPL)) (* _output_get_2 (Variables|InstanceFiled|Get_kPH)) (* _output_get_3 (Variables|InstanceFiled|Get_kD)) (* _output_get_4 (Variables|InstanceFiled|Get_kI)))))
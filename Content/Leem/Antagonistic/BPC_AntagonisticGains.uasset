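; Component that scales left and right arm joint controller stiffness from the expected mass of each side's target obstacle.
; Tick linearly maps expected mass against a per-side maximum to a multiplier, defaulting when zero; real mass is only stored.
; SetMultipliedStiffness multiplies base hand, forearm and arm gains into controller PL gains, though left forearm Y uses the right multiplier.
; Both SafetyRegion references are set to None before being read.
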(event EventBeginPlay
  ;[1 1 1] unity - start
  (Variables|GainsInteractive|SetexpectedMaxMassLeft 0.5)
  (Variables|GainsInteractive|SetexpectedMaxMassRight 0.5))

(event EventTick
  (params (DeltaSeconds :type Float%20%28single-precision%29))
  (Utilities|FlowControl|Sequence
    (:then_0
      (bind _output_get (Variables|Components|SetsafetyRegionRight 0))
      (Variables|Right|SetexpectedMassRight (Variables|/Game/Minjeong/Actor/BP_NewParentObstacle.BP_NewParentObstacle_C|GetExpected%20Mass (Variables|/Game/Minjeong/Component/BPC_ChildSafetyRegionRight.BPC_ChildSafetyRegionRight_C|GettargetObstacle _output_get)))
      (Variables|Right|SetrealMassRight (Variables|/Game/Minjeong/Actor/BP_NewParentObstacle.BP_NewParentObstacle_C|GetReal%20Mass (Variables|/Game/Minjeong/Component/BPC_ChildSafetyRegionRight.BPC_ChildSafetyRegionRight_C|GettargetObstacle _output_get)))
      (if (== (Variables|Right|GetexpectedMassRight) 0.0)
        (Variables|Right|SetstiffnessMultiplierRight 0.5)
        (else
          (Variables|Right|SetstiffnessMultiplierRight (Math|Interpolation|Ease "Linear" (/ (Variables|Right|GetexpectedMassRight) (Variables|GainsInteractive|GetexpectedMaxMassRight)) (Math|Conversions|ToFloat(Integer) "0.05") (Math|Conversions|ToFloat(Integer) "1"))))))
    (:then_1
      (bind _output_get_2 (Variables|Components|SetsafetyRegionLeft 0))
      (Variables|Left|SetexpectedMassLeft (Variables|/Game/Minjeong/Actor/BP_NewParentObstacle.BP_NewParentObstacle_C|GetExpected%20Mass (Variables|/Game/Minjeong/Component/BPC_ChildSafetyRegionLeft.BPC_ChildSafetyRegionLeft_C|GettargetObstacle _output_get_2)))
      (Variables|Left|SetrealMassLeft (Variables|/Game/Minjeong/Actor/BP_NewParentObstacle.BP_NewParentObstacle_C|GetReal%20Mass (Variables|/Game/Minjeong/Component/BPC_ChildSafetyRegionLeft.BPC_ChildSafetyRegionLeft_C|GettargetObstacle _output_get_2)))
      (if (== (Variables|Left|GetexpectedMassLeft) 0.0)
        (Variables|Left|SetstiffnessMultiplierLeft 0.5)
        (else
          (Variables|Left|SetstiffnessMultiplierLeft (Math|Interpolation|Ease "Linear" (/ (Variables|Left|GetexpectedMassLeft) (Variables|GainsInteractive|GetexpectedMaxMassLeft)) (Math|Conversions|ToFloat(Integer) "0.05") (Math|Conversions|ToFloat(Integer) "1"))))))
    (:then_2
      (CallFunction|SetMultipliedStiffness))))

(fn SetMultipliedStiffness
  (bind _lefttarmcontroller_j (Variables|Setting|GetlefttArmController_J))
  (bind _leftforearmcontroller_j (Variables|Setting|GetleftForeArmController_J))
  (bind _righthandcontroller_j (Variables|setting|GetrightHandController_J))
  (bind _rightforearmcontroller_j (Variables|Setting|GetrightForeArmController_J))
  (bind _rightarmcontroller_j (Variables|Setting|GetrightArmController_J))
  (bind _lefthandcontroller_j (Variables|Setting|GetleftHandController_J))
  ;[1 1 1] joint controller 계산
  (Utilities|FlowControl|Sequence
    (:then_0
      ;[1 1 1] set right stiffness
      (Variables|/Game/Leem/Antagonistic/BPC_JointControllerBase.BPC_JointControllerBase_C|SetpLX _righthandcontroller_j (* (Variables|Setting|GethandKLX) (Variables|Right|GetstiffnessMultiplierRight)))
      (Variables|/Game/Leem/Antagonistic/BPC_JointControllerBase.BPC_JointControllerBase_C|SetpLY _righthandcontroller_j (* (Variables|Setting|GethandKLY) (Variables|Right|GetstiffnessMultiplierRight)))
      (Variables|/Game/Leem/Antagonistic/BPC_JointControllerBase.BPC_JointControllerBase_C|SetpLZ _righthandcontroller_j (* (Variables|Setting|GethandKLZ) (Variables|Right|GetstiffnessMultiplierRight)))
      (Variables|/Game/Leem/Antagonistic/BPC_JointControllerBase.BPC_JointControllerBase_C|SetpLX _rightforearmcontroller_j (* (Variables|Setting|GetforeArmKLX) (Variables|Right|GetstiffnessMultiplierRight)))
      (Variables|/Game/Leem/Antagonistic/BPC_JointControllerBase.BPC_JointControllerBase_C|SetpLY _rightforearmcontroller_j (* (Variables|Setting|GetforeArmKLY) (Variables|Right|GetstiffnessMultiplierRight)))
      (Variables|/Game/Leem/Antagonistic/BPC_JointControllerBase.BPC_JointControllerBase_C|SetpLZ _rightforearmcontroller_j (* (Variables|Setting|GetforeArmKLZ) (Variables|Right|GetstiffnessMultiplierRight)))
      (Variables|/Game/Leem/Antagonistic/BPC_JointControllerBase.BPC_JointControllerBase_C|SetpLX _rightarmcontroller_j (* (Variables|Setting|GetarmKLX) (Variables|Right|GetstiffnessMultiplierRight)))
      (Variables|/Game/Leem/Antagonistic/BPC_JointControllerBase.BPC_JointControllerBase_C|SetpLY _rightarmcontroller_j (* (Variables|Setting|GetarmKLY) (Variables|Right|GetstiffnessMultiplierRight)))
      (Variables|/Game/Leem/Antagonistic/BPC_JointControllerBase.BPC_JointControllerBase_C|SetpLZ _rightarmcontroller_j (* (Variables|Setting|GetarmKLZ) (Variables|Right|GetstiffnessMultiplierRight))))
    (:then_1
      ;[1 1 1] set right stiffness
      (Variables|/Game/Leem/Antagonistic/BPC_JointControllerBase.BPC_JointControllerBase_C|SetpLX _lefthandcontroller_j (* (Variables|Setting|GethandKLX) (Variables|Left|GetstiffnessMultiplierLeft)))
      (Variables|/Game/Leem/Antagonistic/BPC_JointControllerBase.BPC_JointControllerBase_C|SetpLY _lefthandcontroller_j (* (Variables|Setting|GethandKLY) (Variables|Left|GetstiffnessMultiplierLeft)))
      (Variables|/Game/Leem/Antagonistic/BPC_JointControllerBase.BPC_JointControllerBase_C|SetpLZ _lefthandcontroller_j (* (Variables|Setting|GethandKLZ) (Variables|Left|GetstiffnessMultiplierLeft)))
      (Variables|/Game/Leem/Antagonistic/BPC_JointControllerBase.BPC_JointControllerBase_C|SetpLX _leftforearmcontroller_j (* (Variables|Setting|GetforeArmKLX) (Variables|Left|GetstiffnessMultiplierLeft)))
      (Variables|/Game/Leem/Antagonistic/BPC_JointControllerBase.BPC_JointControllerBase_C|SetpLY _leftforearmcontroller_j (* (Variables|Setting|GetforeArmKLY) (Variables|Right|GetstiffnessMultiplierRight)))
      (Variables|/Game/Leem/Antagonistic/BPC_JointControllerBase.BPC_JointControllerBase_C|SetpLZ _leftforearmcontroller_j (* (Variables|Setting|GetforeArmKLZ) (Variables|Left|GetstiffnessMultiplierLeft)))
      (Variables|/Game/Leem/Antagonistic/BPC_JointControllerBase.BPC_JointControllerBase_C|SetpLX _lefttarmcontroller_j (* (Variables|Setting|GetarmKLX) (Variables|Left|GetstiffnessMultiplierLeft)))
      (Variables|/Game/Leem/Antagonistic/BPC_JointControllerBase.BPC_JointControllerBase_C|SetpLY _lefttarmcontroller_j (* (Variables|Setting|GetarmKLY) (Variables|Left|GetstiffnessMultiplierLeft)))
      (Variables|/Game/Leem/Antagonistic/BPC_JointControllerBase.BPC_JointControllerBase_C|SetpLZ _lefttarmcontroller_j (* (Variables|Setting|GetarmKLZ) (Variables|Left|GetstiffnessMultiplierLeft))))))
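; Base combat character with punch, kick and throw attacks, blocking that slows walking, and physics-driven hit reactions.
; A combat state machine gates movement and attacks, queuing or chaining combo montages.
; The mesh simulates under PhysicalAnimation; OnHit drops motor strength and applies force, harder on torso bones, and Tick interpolates strength back.
; Per-bone dynamic materials flash on hits and fade; number keys and several unwired graphs hold partial-ragdoll experiments.
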(event Custom|EventHitReaction
  (params (Bone :type Name) (HitLocation :type Vector))
  (Variables|Default|SetHitReactionTimeRemaining (+ (Variables|Default|GetHitReactionTimeRemaining) 2.0))
  (Class|SkeletalMeshComponent|SetAllBodiesBelowSimulatePhysics (Variables|Character|GetMesh) (Utilities|Name|MakeLiteralName "pelvis") true false)
  (Physics|AddImpulse (Variables|Character|GetMesh) HitLocation Bone false) ; Add impulse - direction, velocity
)

(event Custom|EventPhysicalBasedHit
  (Utilities|FlowControl|Delay 1.0)
  (PhysicalAnimation|DeactivatePhysicalAnimation))

(event EventBeginPlay
  (bind _mesh (Variables|Character|GetMesh))
  (bind _physicalanimation (Variables|Default|GetPhysicalAnimation))
  (Class|PhysicalAnimationComponent|SetSkeletalMeshComponent _physicalanimation _mesh)
  (Class|PhysicalAnimationComponent|ApplyPhysicalAnimationSettingsBelow _physicalanimation "root" (Utilities|Struct|MakePhysicalAnimationData false 2e+03 4e+01 2e+03 4e+01) true)
  (Physics|SetSimulatePhysics _mesh true))

(event EventTick
  (params (DeltaSeconds :type Float%20%28single-precision%29))
  (Utilities|FlowControl|Sequence
    (:then_0
      (Combat|Block|UpdateBlockState DeltaSeconds))
    (:then_1
      (Color|UpdateBoneMaterial DeltaSeconds)
      (CallFunction|UpdateStrength DeltaSeconds))))

(event Input|KeyboardEvents|1
  (params (Key :type Key%20Structure))
  (:Pressed
    (Utilities|FlowControl|FlipFlop
      (:A
        (Variables|Anchor|SetAnchorBone "spine_01"))
      (:B
        (Variables|Anchor|SetAnchorBone "spine_01")))))

(event Input|KeyboardEvents|2
  (params (Key :type Key%20Structure))
  (:Pressed
    (Utilities|FlowControl|FlipFlop
      (:A
        (Variables|Anchor|SetAnchorBone "spine_03"))
      (:B
        (Variables|Anchor|SetAnchorBone "spine_01")))))

(event Input|KeyboardEvents|3
  (params (Key :type Key%20Structure))
  (:Pressed
    (Utilities|FlowControl|FlipFlop
      (:A
        (Variables|Anchor|SetAnchorBone "neck_01"))
      (:B
        (Variables|Anchor|SetAnchorBone "spine_01")))))

(event Input|KeyboardEvents|4
  (params (Key :type Key%20Structure))
  (:Pressed
    (Utilities|FlowControl|FlipFlop
      (:A
        (Variables|Anchor|SetAnchorBone "clavicle_l"))
      (:B
        (Variables|Anchor|SetAnchorBone "spine_01")))))

(event Input|KeyboardEvents|5
  (params (Key :type Key%20Structure))
  (:Pressed
    (Utilities|FlowControl|FlipFlop
      (:A
        (Variables|Anchor|SetAnchorBone "upperarm_l"))
      (:B
        (Variables|Anchor|SetAnchorBone "spine_01")))))

(event Input|KeyboardEvents|6
  (params (Key :type Key%20Structure))
  (:Pressed
    (Utilities|FlowControl|FlipFlop
      (:A
        (Variables|Anchor|SetAnchorBone "lowerarm_l"))
      (:B
        (Variables|Anchor|SetAnchorBone "spine_01")))))

(event Input|KeyboardEvents|0
  (params (Key :type Key%20Structure))
  (bind _mesh (Variables|Character|GetMesh))
  (bind _mesh_2 (Variables|Character|GetMesh))
  (bind _mesh_3 (Variables|Character|GetMesh))
  (:Pressed
    (Utilities|FlowControl|FlipFlop
      (:A
        (if (== (Variables|Anchor|GetAnchorBone) "clavicle_l")
          (bind _output_get (Variables|Default|SetIn%20Bone%20Name "clavicle_r"))
          (Class|SkeletalMeshComponent|SetAllBodiesBelowSimulatePhysics _mesh _output_get true true) ; Enable Physics Simulation for some of the Bones
          (Class|SkeletalMeshComponent|SetAllBodiesBelowPhysicsBlendWeight _mesh _output_get (Variables|Anchor|GetBlendingWeight) false true) ; Set the BlendWeight for those Bones
          (elif (== (Variables|Anchor|GetAnchorBone) "upperarm_l")
            (bind _output_get_2 (Variables|Default|SetIn%20Bone%20Name "upperarm_r"))
            (Class|SkeletalMeshComponent|SetAllBodiesBelowSimulatePhysics _mesh_2 _output_get_2 true true) ; Enable Physics Simulation for some of the Bones
            (Class|SkeletalMeshComponent|SetAllBodiesBelowPhysicsBlendWeight _mesh_2 _output_get_2 (Variables|Anchor|GetBlendingWeight) false true) ; Set the BlendWeight for those Bones
            (elif (== (Variables|Anchor|GetAnchorBone) "lowerarm_l")
              (bind _output_get_3 (Variables|Default|SetIn%20Bone%20Name "lowerarm_r"))
              (Class|SkeletalMeshComponent|SetAllBodiesBelowSimulatePhysics _mesh_3 _output_get_3 true true) ; Enable Physics Simulation for some of the Bones
              (Class|SkeletalMeshComponent|SetAllBodiesBelowPhysicsBlendWeight _mesh_3 _output_get_3 (Variables|Anchor|GetBlendingWeight) false true) ; Set the BlendWeight for those Bones
            )))))))

(fn ConstructionScript
  (|CallParentFunction)
  (Color|InitBoneMaterial))

(fn GetAttackMontage
  (switch Utilities|FlowControl|Switch|SwitchonEAttackType (Variables|Combat|Attack|GetCurrentAttackType)
    (:NewEnumerator0
      (LocalVariables|SetReturnValue (Variables|Montage|Attack|GetPunchCombo)))
    (:NewEnumerator1
      (LocalVariables|SetReturnValue (Variables|Montage|Attack|GetKickCombo)))
    (:NewEnumerator4
      (LocalVariables|SetReturnValue (Variables|Montage|Attack|GetThrowAttack))))
  (Math|Integer|IncrementInt (Variables|Combat|Attack|GetComboCount)
    (:%20%20
      (return (LocalVariables|GetReturnValue)))))

(fn ActivatePhysicalAnimation
  (params (StunTime :type Float%20%28double-precision%29))
  (Variables|Default|SetIsPhysicsActive true)
  (Class|PhysicalAnimationComponent|SetStrengthMultiplyer (Variables|Default|GetPhysicalAnimation) 0.0)
  (State|Set|SetCombatState "NewEnumerator5")
  (Variables|Default|SetStunTime StunTime))

(fn DeactivatePhysicalAnimation
  (Class|PhysicalAnimationComponent|SetStrengthMultiplyer (Variables|Default|GetPhysicalAnimation) 1.0)
  (Variables|Default|SetIsPhysicsActive false))

(fn SetBlockState
  (params (IsBlock :type Boolean))
  (Variables|Combat|Block|SetTargetBlock (Math|Float|SelectFloat 1.0 0.0 IsBlock)))

(fn ResetAttackVariables
  (Variables|Combat|Attack|SetComboCount 0)
  (Utilities|Array|Clear (Variables|Combat|Attack|GetPendingMontages))
  (Animation|StopAnimMontage 0)
  (State|Set|SetCombatState "NewEnumerator7"))

(fn InputAttack
  (params (AttackType :type EAttackType%20Enum :default "NewEnumerator0"))
  (bind _attackmontage (Combat|Attack|GetAttackMontage))
  (if (State|Get|CanAttack AttackType)
    (Variables|Combat|Attack|SetCurrentAttackType AttackType)
    (switch Utilities|FlowControl|Switch|SwitchonECombatState (Variables|State|GetCombatState)
      (:NewEnumerator7
        (Animation|PlayAnimMontage _attackmontage 1.0 "None" :!label _label))
      (:NewEnumerator1
        (if (< (Utilities|Array|Length (Variables|Combat|Attack|GetPendingMontages)) 3)
          (Utilities|Array|Add (Variables|Combat|Attack|GetPendingMontages) _attackmontage)))
      (:NewEnumerator2
        (Animation|PlayAnimMontage _attackmontage 1.0 "None"))
      (:NewEnumerator3
        (goto _label))
      (:NewEnumerator8
        (goto _label)))))

(fn HitCharacter
  (params (HitCharacter :type BP%20Character%20Base%20Object%20Reference) (Location :type Vector) (AttackDirection :type AttackDirection%20Enum :default "NewEnumerator0") (BoneName :type Name))
  (if (not (Variables|Combat|Attack|GetIsAttackedInMotion))
    (Variables|Combat|Attack|SetIsAttackedInMotion true)
    (Combat|Hit|AnimationBasedHit HitCharacter BoneName)))

(fn FindHitBoneMaterial
  (params (BoneName :type Name))
  (LocalVariables|SetHitBobeName BoneName)
  (while true
    (if (.ReturnValue (Utilities|Map|Find (Variables|Color|GetBoneMaterial) (LocalVariables|GetHitBobeName)))
      (return (LocalVariables|GetHitBobeName))
      (else
        (LocalVariables|SetHitBobeName (Class|SkinnedMeshComponent|GetParentBone (Variables|Character|GetMesh) (LocalVariables|GetHitBobeName)))))))

(fn ImpactMaterial
  (params (ImpactBone :type Name) (ImpactColor :type Linear%20Color%20Structure) (ImpectTime :type Float%20%28double-precision%29))
  (bind _bonematerial (Variables|Color|GetBoneMaterial))
  (bind _impacttime (Variables|Config|Hit|GetImpactTime))
  (bind (_value _returnvalue) (Utilities|Map|Find _bonematerial ImpactBone))
  (bind _output_get (LocalVariables|SetBoneName ImpactBone))
  (while (and (!= (LocalVariables|GetBoneName) "") (not _returnvalue))
    (LocalVariables|SetBoneName (Class|SkinnedMeshComponent|GetParentBone (Variables|Character|GetMesh) _output_get)))
  (if (!= (LocalVariables|GetBoneName) "")
    (Rendering|Material|SetVectorParameterValue (.instance _value) (Variables|Config|Color|GetBaseColor) ImpactColor :!class /Script/Engine.MaterialInstanceDynamic)
    (Utilities|Map|Add (Variables|Color|GetBoneMaterial) ImpactBone (Utilities|Struct|MakeBoneMaterial (.instance _value) (.basecolor _value) _impacttime (/ 4.0 _impacttime)))))

(fn AnimationBasedHit
  (params (BoneName :type Name))
  (Utilities|FlowControl|Sequence
    (:then_0
      (Combat|Attack|ResetAttackVariables)
      (bind _returnvalue (Combat|Hit|FindHitBoneMaterial BoneName))
      (Color|ImpactMaterial _returnvalue (Variables|Config|Hit|GetHitColor) (Variables|Config|Hit|GetImpactTime)))
    (:then_2
      (Animation|PlayAnimMontage (Variables|Montage|Hit|GetBlockHitMontage) 1.0 "None"))))

(fn CanMove
  (switch Utilities|FlowControl|Switch|SwitchonECombatState (Variables|State|GetCombatState)
    (:NewEnumerator7
      _)
    (:NewEnumerator4
      (return false))
    (:NewEnumerator5
      (return false))
    (:NewEnumerator0
      (Combat|Attack|ResetAttackVariables)
      (Animation|StopAnimMontage 0)
      (State|Set|SetCombatState "NewEnumerator7"))
    (:NewEnumerator1
      (return false))
    (:NewEnumerator2
      (return false))
    (:NewEnumerator3
      _)
    (:NewEnumerator8
      (return false)))
  (return true))

(fn SetCombatState
  (params (State :type ECombatState%20Enum :default "NewEnumerator0"))
  (bind _pendingmontages (Variables|Combat|Attack|GetPendingMontages))
  (switch Utilities|FlowControl|Switch|SwitchonECombatState State
    (:NewEnumerator7
      (Variables|State|SetCombatState State :!label _label))
    (:NewEnumerator4
      (goto _label))
    (:NewEnumerator5
      (Combat|Attack|ResetAttackVariables :!label _label_2)
      (goto _label))
    (:NewEnumerator0
      (goto _label))
    (:NewEnumerator1
      (goto _label))
    (:NewEnumerator2
      (if (Utilities|Array|IsNotEmpty _pendingmontages)
        (Animation|PlayAnimMontage (Utilities|Array|Get(acopy) _pendingmontages) 1.0 "None")
        (Utilities|Array|RemoveIndex _pendingmontages)
        (else
          (goto _label))))
    (:NewEnumerator3
      (goto _label_2))
    (:NewEnumerator8
      (goto _label))))

(fn CanAttack
  (params (AttackType :type EAttackType%20Enum :default "NewEnumerator0"))
  (if (or (Utilities|Enum|Equal(Enum) AttackType "NewEnumerator4") (Utilities|Enum|Equal(Enum) (Variables|State|GetMovementState) "NewEnumerator1"))
    (switch Utilities|FlowControl|Switch|SwitchonECombatState (Variables|State|GetCombatState)
      (:NewEnumerator7
        _)
      (:NewEnumerator4
        (return false))
      (:NewEnumerator5
        (return false))
      (:NewEnumerator0
        (return false))
      (:NewEnumerator1
        (return (Utilities|Enum|Equal(Enum) AttackType (Variables|Combat|Attack|GetCurrentAttackType))))
      (:NewEnumerator2
        (return (Utilities|Enum|Equal(Enum) AttackType (Variables|Combat|Attack|GetCurrentAttackType))))
      (:NewEnumerator3
        _)
      (:NewEnumerator8
        (return (Utilities|Enum|Equal(Enum) AttackType "NewEnumerator3"))))
    (return true)))

(fn UpdateBlockState
  (params (DeltaTime :type Float%20%28double-precision%29))
  (Variables|Combat|Block|SetCurrentBlock (Math|Interpolation|FInterpTo (Variables|Combat|Block|GetCurrentBlock) (Variables|Combat|Block|GetTargetBlock) DeltaTime (Variables|Config|Combat|Block|GetBlockInterpSpeed)))
  (Variables|/Script/Engine.CharacterMovementComponent|SetMaxWalkSpeed (Variables|Character|GetCharacterMovement) (- (Variables|Config|Movement|GetWalkSpeed) (* (Math|Interpolation|FInterpTo (Variables|Combat|Block|GetCurrentBlock) (Variables|Combat|Block|GetTargetBlock) DeltaTime (Variables|Config|Combat|Block|GetBlockInterpSpeed)) (Variables|Config|Movement|GetBlockWalkSpeedDiff)))))

(fn IsBlock
  (return (> (Variables|Combat|Block|GetCurrentBlock) 0.5)))

(fn SetMovementState
  (params (MovementState :type EMovementState%20Enum :default "NewEnumerator0"))
  (bind _output_get (Variables|State|SetMovementState MovementState))
  (switch Utilities|FlowControl|Switch|SwitchonEMovementState _output_get
    (:NewEnumerator0
      (Variables|Default|SetbUseControllerRotationYaw false))
    (:NewEnumerator1
      (Variables|Default|SetbUseControllerRotationYaw true))))

(fn InitBoneMaterial
  (Color|CreateBoneMaterialbyColor (Utilities|Array|MakeArray (Utilities|Struct|MakeCharacterMaterialInfo "head" 13) (Utilities|Struct|MakeCharacterMaterialInfo "neck_01" 12) (Utilities|Struct|MakeCharacterMaterialInfo "lowerarm_l" 6) (Utilities|Struct|MakeCharacterMaterialInfo "hand_l" 7) (Utilities|Struct|MakeCharacterMaterialInfo "upperarm_r" 10) (Utilities|Struct|MakeCharacterMaterialInfo "hand_r" 11)) (Variables|Color|GetBase))
  (Color|CreateBoneMaterialbyColor (Utilities|Array|MakeArray (Utilities|Struct|MakeCharacterMaterialInfo "pelvis" 0) (Utilities|Struct|MakeCharacterMaterialInfo "spine_01" 1) (Utilities|Struct|MakeCharacterMaterialInfo "spine_02" 2) (Utilities|Struct|MakeCharacterMaterialInfo "spine_03" 3) (Utilities|Struct|MakeCharacterMaterialInfo "clavicle_l" 4) (Utilities|Struct|MakeCharacterMaterialInfo "upperarm_l" 5) (Utilities|Struct|MakeCharacterMaterialInfo "calvicle_r" 8) (Utilities|Struct|MakeCharacterMaterialInfo "upperarm_r" 9)) (Variables|Color|GetUpperBody))
  (Color|CreateBoneMaterialbyColor (Utilities|Array|MakeArray (Utilities|Struct|MakeCharacterMaterialInfo "thigh_l" 15) (Utilities|Struct|MakeCharacterMaterialInfo "calf_l" 16) (Utilities|Struct|MakeCharacterMaterialInfo "thigh_r" 18) (Utilities|Struct|MakeCharacterMaterialInfo "calf_r" 19)) (Variables|Color|GetLowerBody))
  (Color|CreateBoneMaterialbyColor (Utilities|Array|MakeArray (Utilities|Struct|MakeCharacterMaterialInfo "foot_l" 17) (Utilities|Struct|MakeCharacterMaterialInfo "foot_r" 20)) (Variables|Color|GetFeet)))

(fn CreateBoneMaterialbyColor
  (params (MaterialInfos :type Array%20of%20Character%20Material%20Info%20Structures) (color :type Linear%20Color%20Structure))
  (for _array_element MaterialInfos
    (bind _returnvalue (Rendering|Material|CreateDynamicMaterialInstance (Variables|Character|GetMesh) (.materialindex _array_element) 0 "None" :!class /Script/Engine.PrimitiveComponent))
    (Rendering|Material|SetVectorParameterValue _returnvalue "BaseColor" color :!class /Script/Engine.MaterialInstanceDynamic)
    (Utilities|Map|Add (Variables|Color|GetBoneMaterial) (.bonename _array_element) (Utilities|Struct|MakeBoneMaterial _returnvalue color 0.0 0.0))))

(fn UpdateBoneMaterial
  (params (DeltaTime :type Float%20%28double-precision%29))
  (bind _bonematerial (Variables|Color|GetBoneMaterial))
  (bind _keys (Utilities|Map|Keys (Variables|Color|GetBoneMaterial)))
  (for _array_element _keys
    (Utilities|Map|Add _bonematerial _array_element (Utilities|Struct|MakeBoneMaterial (.instance (.Value (Utilities|Map|Find _bonematerial _array_element))) (.basecolor (.Value (Utilities|Map|Find _bonematerial _array_element))) (- (.impacttime (.Value (Utilities|Map|Find _bonematerial _array_element))) DeltaTime) (.impactspeed (.Value (Utilities|Map|Find _bonematerial _array_element)))))
    (if (> (- (.impacttime (.Value (Utilities|Map|Find _bonematerial _array_element))) DeltaTime) 0.0)
      (bind _returnvalue (Rendering|Material|GetVectorParameterValue (.instance (.Value (Utilities|Map|Find _bonematerial _array_element))) (Variables|Config|Color|GetBaseColor) :!class /Script/Engine.MaterialInstanceDynamic))
      (Rendering|Material|SetVectorParameterValue (.instance (.Value (Utilities|Map|Find _bonematerial _array_element))) (Variables|Config|Color|GetBaseColor) (Class|KismetMathLibrary|CInterpto _returnvalue (.basecolor (.Value (Utilities|Map|Find _bonematerial _array_element))) DeltaTime (.impactspeed (.Value (Utilities|Map|Find _bonematerial _array_element)))) :!class /Script/Engine.MaterialInstanceDynamic))))

(fn PhysicalBasedHit
  (params (BoneName :type Name) (ImpactDirection :type Vector) (StunTime :type Float%20%28double-precision%29) (Power :type Float%20%28double-precision%29))
  (bind _returnvalue (Math|Vector|Normalize ImpactDirection))
  (bind _mesh (Variables|Character|GetMesh))
  (bind _returnvalue_2 (* _returnvalue Power))
  (if (Math|Boolean|ORBoolean (== BoneName "pelvis") (== BoneName "spine_01") (== BoneName "spine_02") (== BoneName "spine_03"))
    (State|Set|SetCombatState "NewEnumerator5")
    (PhysicalAnimation|ActivatePhysicalAnimation StunTime)
    (Physics|AddForce _mesh (* _returnvalue_2 5e+05) BoneName true)
    (Variables|Default|SetInterpSpeed 0.1)
    (else
      (Class|PhysicalAnimationComponent|SetStrengthMultiplyer (Variables|Default|GetPhysicalAnimation) 0.01)
      (Physics|AddForce _mesh (* _returnvalue_2 1e+05) BoneName true)
      (Variables|Default|SetInterpSpeed 0.4))))

(fn OnHit
  (params (BoneName :type Name) (ImpactNormal :type Vector) (LaunchDirection :type Vector))
  (Combat|Attack|ResetAttackVariables)
  (bind _returnvalue (Combat|Hit|FindHitBoneMaterial BoneName))
  (Color|ImpactMaterial _returnvalue (Variables|Config|Hit|GetHitColor) (Variables|Config|Hit|GetImpactTime))
  (Combat|Hit|PhysicalBasedHit BoneName ImpactNormal 0.5 1.0))

(fn UpdateSimulate
  (params (DeltaTime :type Float%20%28double-precision%29))
  (bind _keys (Utilities|Map|Keys (Variables|Default|GetHitPhysics)))
  (for _array_element _keys
    (LocalVariables|SetLoopBoneName _array_element)
    (bind _output_get (LocalVariables|SetLoopBlend (Math|Interpolation|FInterpTo (.Value (Utilities|Map|Find (Variables|Default|GetHitPhysics) (LocalVariables|GetLoopBoneName))) 0.0 DeltaTime 1.0)))
    (if (> _output_get 0.0)
      (Utilities|Map|Add (Variables|Default|GetHitPhysics) (LocalVariables|GetLoopBoneName) (LocalVariables|GetLoopBlend))
      (Class|SkeletalMeshComponent|SetAllBodiesBelowPhysicsBlendWeight (Variables|Character|GetMesh) (LocalVariables|GetLoopBoneName) (LocalVariables|GetLoopBlend) false true)
      (else
        (Utilities|Array|Add (LocalVariables|GetWillRemove) (LocalVariables|GetLoopBoneName)))))
  (for _array_element_2 (LocalVariables|GetWillRemove)
    (Utilities|Map|Remove (Variables|Default|GetHitPhysics) _array_element_2))
  (Utilities|Array|Clear (LocalVariables|GetWillRemove)))

(fn PhysicsHit
  (params (BoneName :type Name) (Force :type Vector))
  (bind _mesh (Variables|Character|GetMesh))
  (bind _mesh_2 (Variables|Character|GetMesh))
  (bind _returnvalue (Class|SkinnedMeshComponent|GetParentBone _mesh BoneName))
  (bind _returnvalue_2 (Class|SkinnedMeshComponent|GetParentBone _mesh_2 _returnvalue))
  (if (or (== _returnvalue "") (== _returnvalue "root"))
    (Utilities|Map|Add (Variables|Default|GetHitPhysics) BoneName 1.0)
    (Physics|AddForce (Variables|Character|GetMesh) Force BoneName false)
    (elif (or (== _returnvalue_2 "") (== _returnvalue_2 "root"))
      (Utilities|Map|Add (Variables|Default|GetHitPhysics) _returnvalue 1.0)
      (Physics|AddForce (Variables|Character|GetMesh) Force BoneName false)
      (else
        (Utilities|Map|Add (Variables|Default|GetHitPhysics) _returnvalue_2 1.0)
        (Physics|AddForce (Variables|Character|GetMesh) Force BoneName false)))))

(fn UpdateStrength
  (params (DeltaTime :type Float%20%28double-precision%29))
  (bind _mesh (Variables|Character|GetMesh))
  (bind _physicalanimation (Variables|Default|GetPhysicalAnimation))
  (bind _interpspeed (Variables|Default|GetInterpSpeed))
  (bind _returnvalue (Transformation|GetSocketLocation _mesh "pelvis"))
  (bind _strengthmultiplyer (Variables|/Script/Engine.PhysicalAnimationComponent|GetStrengthMultiplyer _physicalanimation))
  (bind _returnvalue_2 (Math|Interpolation|FInterpTo _strengthmultiplyer 1.0 DeltaTime _interpspeed))
  (if (> (Variables|Default|GetStunTime) 0.0)
    (Variables|Default|SetStunTime (- (Variables|Default|GetStunTime) DeltaTime))
    (Transformation|SetActorLocation (Math|Vector|MakeVector (.x _returnvalue) (.y _returnvalue) (.z (Transformation|GetActorLocation))) false false :!label _label)
    (elif (< _strengthmultiplyer 1.0)
      (Class|PhysicalAnimationComponent|SetStrengthMultiplyer _physicalanimation _returnvalue_2)
      (if (< _returnvalue_2 0.1)
        (goto _label)
        (else
          (State|Set|SetCombatState "NewEnumerator7")
          (Class|PhysicalAnimationComponent|SetStrengthMultiplyer (Variables|Default|GetPhysicalAnimation) 1.0))))))

(fn Throw
  (bind _returnvalue (Game|SpawnActorfromClass "/Game/Leem/BP_ThrowObject.BP_ThrowObject_C" (Math|Transform|MakeTransform (Transformation|GetWorldLocation (Variables|Default|GetSphere_0)) (Transformation|GetWorldRotation (Variables|Character|GetMesh)) "1.000000,1.000000,1.000000") "Undefined" 0 0))
  (Physics|SetPhysicsLinearVelocity (Variables|/Game/Leem/BP_ThrowObject.BP_ThrowObject_C|Getcollision _returnvalue) (* (Math|Vector|Normalize (Math|Vector|MakeVector (.x (Math|Vector|GetUnitDirection(Vector) (Transformation|GetActorLocation) (Transformation|GetActorLocation _returnvalue))) (.y (Math|Vector|GetUnitDirection(Vector) (Transformation|GetActorLocation) (Transformation|GetActorLocation _returnvalue))) (* (.z (Math|Vector|GetUnitDirection(Vector) (Transformation|GetActorLocation) (Transformation|GetActorLocation _returnvalue))) 0.4))) 2e+03) false "None"))
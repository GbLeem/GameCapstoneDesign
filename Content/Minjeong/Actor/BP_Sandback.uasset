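; BP_Sandback is a world actor with a toggleable highlight outline, built on a parent class that supplies the outline functions.
; On BeginPlay it snaps SimulateStatic1 to SimulateStatic's world transform.
; CreateOutline puts a dynamic M_Outline_Inst material on SimulateStatic, and DeleteOutline restores MI_Pillar_1, with HasOutline guarding both.
; The overlap event checks the player's IsRegionActive but takes no action.
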(event EventBeginPlay
  (|CallParentFunction)
  (Transformation|SetWorldTransform (Variables|Default|GetSimulateStatic1) (Transformation|GetWorldTransform (Variables|Default|GetSimulateStatic)) false false))

(event Collision|EventActorBeginOverlap
  (params (OtherActor :type Actor%20Object%20Reference))
  (bind _asbp_player (Utilities|Casting|CastToBP_Player (Game|Player|GetPlayerPawn 0)))
  (if (Variables|/Game/Character/BP_Player.BP_Player_C|GetisRegionActive _asbp_player)
    _))

(event EventTick
  (params (DeltaSeconds :type Float%20%28single-precision%29))
  (|CallParentFunction DeltaSeconds) ; 지금 이 노드는 비활성 상태입니다. \n핀을 끌어서 다른 노드를 연결하면 활성화됩니다.
)

(fn ConstructionScript
  (|CallParentFunction))

(fn CreateOutline
  (|CallParentFunction)
  (if (not (Variables|Default|GetHasOutline))
    (bind _returnvalue (Rendering|Material|CreateDynamicMaterialInstance (Variables|Default|GetSimulateStatic) 0 "/Game/Minjeong/SafetyRegionEffect/Outline/M_Outline_Inst.M_Outline_Inst" "None" :!class /Script/Engine.PrimitiveComponent))
    (bind _output_get (Variables|Default|SetDMI _returnvalue))
    (Rendering|Material|SetScalarParameterValue _output_get "Scale" 3.0 :!class /Script/Engine.MaterialInstanceDynamic)
    (Variables|Default|SetHasOutline true)))

(fn DeleteOutline
  (bind _dmi (Variables|Default|GetDMI))
  (|CallParentFunction)
  (if (Variables|Default|GetHasOutline)
    (Rendering|Material|SetScalarParameterValue _dmi "scale" 0.0 :!class /Script/Engine.MaterialInstanceDynamic)
    (Rendering|Material|SetVectorParameterValue _dmi "color" (Utilities|Struct|MakeLinearColor 0.0 0.0 0.0 0.0) :!class /Script/Engine.MaterialInstanceDynamic)
    (Rendering|Material|SetMaterial (Variables|Default|GetSimulateStatic) 0 "/Game/FunObstacleCourse/Mesh/Materials/MI_Pillar_1.MI_Pillar_1")
    (Variables|Default|SetHasOutline false)))
(event EventBeginPlay
  (|CallParentFunction)
  (bind _location (Timeline|Timeline_0 PlayFromStart)
    (:Update
      (Transformation|SetRelativeLocation (Variables|Default|GetPillar_2) (Math|Vector|MakeVector -1e+02 _location 0.0) false false))))

(event Collision|EventActorBeginOverlap
  (params (OtherActor :type Actor%20Object%20Reference)))

(event EventTick
  (params (DeltaSeconds :type Float%20%28single-precision%29))
  (|CallParentFunction DeltaSeconds)
  (Transformation|SetWorldTransform (Variables|Default|GetStaticMesh) (Transformation|GetWorldTransform (Variables|Default|GetPillar_2)) false false))

(fn ConstructionScript
  (|CallParentFunction))

(fn CreateOutline
  (|CallParentFunction)
  (if (not (Variables|Default|GetHasOutline))
    (bind _returnvalue (Rendering|Material|CreateDynamicMaterialInstance (Variables|Default|GetPillar_2) 0 "/Game/Minjeong/SafetyRegionEffect/Outline/M_Outline_Inst.M_Outline_Inst" "None" :!class /Script/Engine.PrimitiveComponent))
    (bind _output_get (Variables|Default|SetDMI _returnvalue))
    (Rendering|Material|SetScalarParameterValue _output_get "Scale" 3.0 :!class /Script/Engine.MaterialInstanceDynamic)
    (Variables|Default|SetHasOutline true)))

(fn DeleteOutline
  (bind _dmi (Variables|Default|GetDMI))
  (|CallParentFunction)
  (if (Variables|Default|GetHasOutline)
    (Rendering|Material|SetScalarParameterValue _dmi "scale" 0.0 :!class /Script/Engine.MaterialInstanceDynamic)
    (Rendering|Material|SetVectorParameterValue _dmi "color" (Utilities|Struct|MakeLinearColor 0.0 0.0 0.0 0.0) :!class /Script/Engine.MaterialInstanceDynamic)
    (Rendering|Material|SetMaterial (Variables|Default|GetPillar_2) 0 "/Game/FunObstacleCourse/Mesh/Materials/MI_Pillar_2.MI_Pillar_2")
    (Variables|Default|SetHasOutline false)))
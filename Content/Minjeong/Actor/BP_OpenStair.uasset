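; BP_OpenStair is an actor that slides a stair ramp mesh once the player has triggered opening.
; Each Tick it casts the player pawn to BP_Player and polls its IsOpen flag.
; While that flag is set, it nudges SMRamp3 along negative relative X by a fixed, frame-rate-dependent step, incrementing Count until a limit stops the movement.
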(event EventBeginPlay)

(event Collision|EventActorBeginOverlap
  (params (OtherActor :type Actor%20Object%20Reference)))

(event EventTick
  (params (DeltaSeconds :type Float%20%28single-precision%29))
  ;[1 1 1] Player 에서 Enter bool 받아서 Add Location
  (bind _asbp_player (Utilities|Casting|CastToBP_Player (Game|Player|GetPlayerPawn 0)))
  (if (Variables|/Game/Character/BP_Player.BP_Player_C|GetIsOpen _asbp_player)
    (if (<= (Variables|Default|GetCount) 4e+01)
      (Transformation|AddRelativeLocation (Variables|Default|GetSM_Ramp_3) "-2.000000, 0, 0" false false)
      (Variables|Default|SetCount (+ (Variables|Default|GetCount) 0.1)))))

(fn ConstructionScript)
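; Child obstacle that swings its Base back and forth in pitch and knocks the player on overlap.
; Two timelines drive the rotation, handing off through three-second delays started from their updates.
; Tick polls player overlap, deactivating physical animation if the player's region is active, otherwise activating it and applying a stunning pelvis hit.
; Outline functions add a dynamic outline material to One0 and later restore its ball material.
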(event EventBeginPlay
  (|CallParentFunction)
  (bind _새_트랙_0 (Timeline|Timeline_0 Play)
    (:Update
      (Transformation|SetRelativeRotation (Variables|Default|Getbase) (Math|Rotator|MakeRotator 0.0 _새_트랙_0 0.0) false false)
      (Utilities|FlowControl|Delay 3.0)
      (bind _새_트랙_0_2 (Timeline|Timeline_1 ReverseFromEnd)
        (:Update
          (Transformation|SetRelativeRotation (Variables|Default|Getbase) (Math|Rotator|MakeRotator 0.0 _새_트랙_0_2 0.0) false false)
          (Utilities|FlowControl|Delay 3.0)
          (Timeline|Timeline_0 Play))))))

(event EventTick
  (params (DeltaSeconds :type Float%20%28single-precision%29))
  (|CallParentFunction DeltaSeconds)
  (if (Collision|IsOverlappingActor (Game|Player|GetPlayerPawn 0) :!class /Script/Engine.Actor)
    (bind _asbp_player (Utilities|Casting|CastToBP_Player (Game|Player|GetPlayerPawn 0)))
    (if (Variables|/Game/Character/BP_Player.BP_Player_C|GetisRegionActive _asbp_player)
      (Default|DeactivatePhysicalAnimation _asbp_player)
      (else
        (Default|ActivatePhysicalAnimation _asbp_player 0.25)
        (Default|PhysicalBasedHit _asbp_player "pelvis" (* (Math|Vector|GetForwardVector (Math|Rotator|MakeRotator (.roll (Math|Rotator|FindLookatRotation (Transformation|GetActorLocation) (Transformation|GetActorLocation _asbp_player))) 0.0 0.0)) (Variables|Default|Getminus)) 2.0 0.1)))))

(fn ConstructionScript
  (|CallParentFunction))

(fn CreateOutline
  ;[1 1 1] Create Outline
  (if (not (Variables|Default|GetHasOutline))
    (bind _returnvalue (Rendering|Material|CreateDynamicMaterialInstance (Variables|Default|Getone_0) 0 "/Game/Minjeong/SafetyRegionEffect/Outline/M_Outline_Inst.M_Outline_Inst" "None" :!class /Script/Engine.PrimitiveComponent))
    (bind _output_get (Variables|Default|SetDMI _returnvalue))
    (Rendering|Material|SetScalarParameterValue _output_get "Scale" 3.0 :!class /Script/Engine.MaterialInstanceDynamic)
    (Variables|Default|SetHasOutline true)))

(fn DeleteOutline
  (bind _dmi (Variables|Default|GetDMI))
  ;[1 1 1] Delete Outline
  (if (Variables|Default|GetHasOutline)
    (Rendering|Material|SetScalarParameterValue _dmi "scale" 0.0 :!class /Script/Engine.MaterialInstanceDynamic)
    (Rendering|Material|SetVectorParameterValue _dmi "color" (Utilities|Struct|MakeLinearColor 0.0 0.0 0.0 0.0) :!class /Script/Engine.MaterialInstanceDynamic)
    (Rendering|Material|SetMaterial (Variables|Default|Getone_0) 0 "/Game/FunObstacleCourse/Mesh/Materials/MI_Ball_1.MI_Ball_1")
    (Variables|Default|SetHasOutline false)))
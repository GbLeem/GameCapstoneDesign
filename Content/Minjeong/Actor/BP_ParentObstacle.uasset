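; Base obstacle actor that takes its static mesh from the DT_Obstacle row at index ID, set on construction and again at BeginPlay.
; Each tick it records squared velocity and mesh mass, copying them into the expected values when the matching flags are set.
; An ObstacleLocation event stores a location and distance.
; Skeletal mesh and offset nodes in InitMesh are unconnected.
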(event Custom|ObstacleLocation
  (params (location :type Vector) (distance :type Float%20%28double-precision%29))
  (Variables|Default|SetLocation location)
  (Variables|Default|SetDistance distance))

(event EventBeginPlay
  (CallFunction|InitMesh))

(event EventTick
  (params (DeltaSeconds :type Float%20%28single-precision%29))
  (Variables|Default|SetReal%20Velocity (Math|Vector|VectorLengthSquared (Transformation|GetVelocity)))
  (Variables|Default|SetReal%20Mass (Physics|GetMass (Variables|Default|GetStaticMesh)))
  (if (Variables|Default|GetsetSmaeMass)
    (Variables|Default|SetExpected%20Mass (Variables|Default|GetReal%20Mass)))
  (if (Variables|Default|GetsetSameVelocity)
    (Variables|Default|SetExpected%20Velocity (Variables|Default|GetReal%20Velocity))))

(fn ConstructionScript
  (CallFunction|InitMesh))

(fn InitMesh
  (bind _outrownames (DataTable|GetDataTableRowNames "/Game/Minjeong/DataTables/DT_Obstacle.DT_Obstacle"))
  (bind _returnvalue (Utilities|GetDataTableRow "/Game/Minjeong/DataTables/DT_Obstacle.DT_Obstacle" (Utilities|Array|Get(acopy) _outrownames (Variables|Default|GetID))) ; Row Name으로부터 데이터 테이블 한 행 얻음
    (:then
      (Components|StaticMesh|SetStaticMesh (Variables|Default|GetStaticMesh) (.StaticMesh (Utilities|Struct|BreakS_ItemMesh (.Mesh (Utilities|Struct|BreakS_Obstacle _returnvalue))))))
    (:RowNotFound
      (return))))
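; BP_WithoutTire is an actor that repeatedly launches BP_Ball projectiles.
; A Delay on Tick paces it to roughly one ball every two seconds, spawned at the Arrow component's transform.
; Each ball's mesh gets a physics velocity pointing from the actor's origin through the spawn point, then CallDetroyBall is invoked on it.
; The Destory function is an empty stub.
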(event EventBeginPlay)

(event Collision|EventActorBeginOverlap
  (params (OtherActor :type Actor%20Object%20Reference)))

(event EventTick
  (params (DeltaSeconds :type Float%20%28single-precision%29))
  (Utilities|FlowControl|Delay 2.0)
  (bind _returnvalue (Game|SpawnActorfromClass "/Game/Minjeong/Actor/NoInteractionActor/BP_Ball.BP_Ball_C" (Math|Transform|MakeTransform (Transformation|GetWorldLocation (Variables|Default|GetArrow)) (Transformation|GetWorldRotation (Variables|Default|GetArrow)) "1.000000,1.000000,1.000000") "Undefined" 0 0))
  (Physics|SetPhysicsLinearVelocity (Variables|/Game/Minjeong/Actor/NoInteractionActor/BP_Ball.BP_Ball_C|GetStaticMesh _returnvalue) (* (Math|Vector|GetUnitDirection(Vector) (Transformation|GetActorLocation) (Transformation|GetActorLocation _returnvalue)) 1e+03) false "None")
  (Default|CallDetroyBall _returnvalue))

(fn ConstructionScript)

(fn Destory)
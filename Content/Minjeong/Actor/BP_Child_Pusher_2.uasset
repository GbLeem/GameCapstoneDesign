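; Pusher hazard child Blueprint: a pillar that moves along relative Z and knocks back the player on contact.
; On BeginPlay, a speed timeline scaled by PusherSpeed sets the motion timeline's play rate, while Static1 copies the pillar's transform each tick.
; Tick polls player overlap, triggering a physical-animation hit with stun, or deactivating physical animation if IsRegionActive.
; Outline overrides swap the pillar between a dynamic outline material and its original.
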(event EventBeginPlay
  (|CallParentFunction)
  (bind _speed (Timeline|Timeline_1 PlayFromStart)
    (:Update
      (Components|Timeline|SetPlayRate (Variables|Default|GetTimeline_0) (* _speed (Variables|Default|GetPusherSpeed)))
      (bind _location (Timeline|Timeline_0 PlayFromStart)
        (:Update
          (Transformation|SetRelativeLocation (Variables|Default|GetPillar_1) (Math|Vector|MakeVector 0.0 0.0 _location) false false))))))

(event Collision|EventActorBeginOverlap
  (params (OtherActor :type Actor%20Object%20Reference)))

(event EventTick
  (params (DeltaSeconds :type Float%20%28single-precision%29))
  (|CallParentFunction DeltaSeconds)
  (Transformation|SetWorldTransform (Variables|Default|GetStatic1) (Transformation|GetWorldTransform (Variables|Default|GetPillar_1)) false false)
  (if (Collision|IsOverlappingActor (Variables|Default|GetPillar_1) (Game|Player|GetPlayerPawn 0) :!class /Script/Engine.PrimitiveComponent)
    (bind _asbp_player (Utilities|Casting|CastToBP_Player (Game|Player|GetPlayerPawn 0)))
    (if (Variables|/Game/Character/BP_Player.BP_Player_C|GetisRegionActive _asbp_player)
      (Default|DeactivatePhysicalAnimation _asbp_player)
      (else
        (Default|ActivatePhysicalAnimation _asbp_player 0.25)
        (Default|PhysicalBasedHit _asbp_player "pelvis" (* (Math|Vector|GetForwardVector (Math|Rotator|MakeRotator (.roll (Math|Rotator|FindLookatRotation (Transformation|GetActorLocation) (Transformation|GetActorLocation _asbp_player))) 0.0 0.0)) (Variables|Default|Getminus)) 2.0 0.5)))))

(fn ConstructionScript
  (|CallParentFunction))

(fn CreateOutline
  (|CallParentFunction)
  (if (not (Variables|Default|GetHasOutline))
    (bind _returnvalue (Rendering|Material|CreateDynamicMaterialInstance (Variables|Default|GetPillar_1) 0 "/Game/Minjeong/SafetyRegionEffect/Outline/M_Outline_Inst.M_Outline_Inst" "None" :!class /Script/Engine.PrimitiveComponent))
    (bind _output_get (Variables|Default|SetDMI _returnvalue))
    (Rendering|Material|SetScalarParameterValue _output_get "Scale" 3.0 :!class /Script/Engine.MaterialInstanceDynamic)
    (Rendering|Material|SetVectorParameterValue _output_get "None" "(R=0.000000,G=0.133333,B=1.000000,A=1.000000)" :!class /Script/Engine.MaterialInstanceDynamic)
    (Variables|Default|SetHasOutline true)))

(fn DeleteOutline
  (bind _dmi (Variables|Default|GetDMI))
  (|CallParentFunction)
  (if (Variables|Default|GetHasOutline)
    (Rendering|Material|SetScalarParameterValue _dmi "scale" 0.0 :!class /Script/Engine.MaterialInstanceDynamic)
    (Rendering|Material|SetVectorParameterValue _dmi "color" (Utilities|Struct|MakeLinearColor 0.0 0.0 0.0 0.0) :!class /Script/Engine.MaterialInstanceDynamic)
    (Rendering|Material|SetMaterial (Variables|Default|GetPillar_1) 0 "/Game/FunObstacleCourse/Mesh/Materials/MI_Pillar_1.MI_Pillar_1")
    (Variables|Default|SetHasOutline false)))
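; BPC_SafetyRegionBase is a component that holds shared data for the player's left and right safety regions, apparently as a base for safety-region logic.
; BeginPlay sets default origin offset, region radius and reaction time, none of which are used in this graph.
; Every Tick it casts the first player pawn to BP_Player and copies both safety region components' world transforms into its origin region variables.
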(event EventBeginPlay
  (Variables|SettingsINTERACTIVE|SetoriginOffset "0.100000,2.000000,0.600000")
  (Variables|SettingsINTERACTIVE|SetradiusRegion 6e+01)
  (Variables|SettingsINTERACTIVE|SetreactionTime 0.1))

(event EventTick
  (params (DeltaSeconds :type Float%20%28single-precision%29))
  ;[1 1 1] Left/Right Safety Region 위치값 Origin Region으로 업데이트
  (bind _asbp_player (Utilities|Casting|CastToBP_Player (Game|Player|GetPlayerPawn 0)))
  (Variables|SettingsINTERACTIVE|SetoriginLeftRegion (Transformation|GetWorldTransform (Variables|/Game/Character/BP_Player.BP_Player_C|GetLeftSafetyRegion _asbp_player)))
  (Variables|SettingsINTERACTIVE|SetoriginRightRegion (Transformation|GetWorldTransform (Variables|/Game/Character/BP_Player.BP_Player_C|GetRightSafetyRegion _asbp_player))))
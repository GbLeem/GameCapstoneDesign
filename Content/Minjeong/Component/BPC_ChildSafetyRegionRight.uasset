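; Right-side safety region component that computes a protective right-hand IK target against nearby obstacles from the player's right trigger events, which it rebinds every Tick.
; Enter and Stay trace from the region origin to record obstacle hits, and Stay selects the nearest.
; The hit plus a mesh-relative offset becomes the fixed target, with Static/Dynamic tag handling.
; Movement-in/out flags track transitions, restarting on obstacle changes and reversing when none remain.
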(event EventBeginPlay
  (|CallParentFunction)
  (bind _asbp_player (Utilities|Casting|CastToBP_Player (Game|Player|GetPlayerPawn 0))))

(event EventTick
  (params (DeltaSeconds :type Float%20%28single-precision%29))
  (|CallParentFunction DeltaSeconds)
  (EventDispatchers|BindEventtoOnTriggerEnterRight (stale EventBeginPlay _asbp_player) (delegate EnterEventGraph))
  (EventDispatchers|BindEventtoOnTriggerStayRight (stale EventBeginPlay _asbp_player) (delegate StayEventGraph))
  (EventDispatchers|BindEventtoOnTriggerEndRight (stale EventBeginPlay _asbp_player) (delegate EndEventGraph)))

(fn IncreaseSpring)

(fn SetOffset
  (bind _asbp_player (Utilities|Casting|CastToBP_Player (Game|Player|GetPlayerPawn 0)))
  (bind _output_get (Variables|Default|Setoffset (+ (* (Math|Vector|GetUpVector (Variables|/Script/Engine.Character|GetMesh _asbp_player)) (.y (Variables|RightHand-Hit|GethitOffsetRight))) (* (Math|Vector|GetRightVector (Variables|/Script/Engine.Character|GetMesh _asbp_player)) (.x (Variables|RightHand-Hit|GethitOffsetRight))) (* (Math|Vector|GetForwardVector (Variables|/Script/Engine.Character|GetMesh _asbp_player)) (.z (Variables|RightHand-Hit|GethitOffsetRight))))))
  (return _output_get))

(event Custom|OnTriggerEnterEvent
  (params (other :type BP%20New%20Parent%20Obstacle%20Object%20Reference) (postion :type Vector) (ID :type Integer))
  (if (Variables|HandSpring|GetmodifySpring)
    (Utilities|Time|SetTimerbyFunctionName 0 "IncreaseSpring" 0.0)
    (else
      (bind _s_obstacle (CallFunction|ObstacleIDtoStruct ID))
      (if (Utilities|Enum|NotEqual(Enum) (.Tag (Utilities|Struct|BreakS_Obstacle _s_obstacle)) "NewEnumerator2")
        (Variables|RightHand-Hit|SetraycastOriginRight (.location (Variables|Default|GetoriginRightRegion))) ; We protect the origin, and get the closest point in the external object to the previous body part to protect
        (bind _offset (CallFunction|SetOffset))
        (Variables|Default|Setoffset _offset) ; Create an offset, in case it is necessary
        (if (== (Utilities|Array|Length (Variables|RightHand-Obstacles|Getobstacles)) 0) ; For the first obstacle, the list is empty at this point
          ;[1 1 1] // Start moving to the target
          (Variables|RightHand-Debug|SethasRightStartedMovingIn true)
          (Variables|RightHand-Debug|SethasRightStartedMovingOut false)
          (Variables|RightHand-Debug|SethasRightTargetReached false)
          (bind _outhit (Collision|LineTraceByChannel (Variables|RightHand-Hit|GetraycastOriginRight) postion "TraceTypeQuery1" false 0 "None"))
          (Default|ObstacleLocation other (.location _outhit) (.distance _outhit))
          (Utilities|Array|Add (Variables|RightHand-Obstacles|Getobstacles) other))))))

(event Custom|OnTirggerStayEvent
  (params (Other :type BP%20New%20Parent%20Obstacle%20Object%20Reference) (Position :type Vector) (ID :type Integer))
  (Variables|EventParam|SetPositionStay Position)
  (bind _s_obstacle (CallFunction|ObstacleIDtoStruct ID))
  (if (Utilities|Enum|NotEqual(Enum) (.Tag (Utilities|Struct|BreakS_Obstacle _s_obstacle)) "NewEnumerator2")
    ;[1 1 1] Origin Region 위치시작-물체 남은위치 끝까지
    (bind _output_get (Variables|RightHand-Hit|SetraycastOriginRight (.location (Variables|Default|GetoriginRightRegion)))) ; We protect the origin, and get the closest point in the external object to the previous body part to protect
    (bind _outhit (Collision|SphereTraceByChannel _output_get (Variables|EventParam|GetPositionStay) 0.0 "TraceTypeQuery1" false 0 "None" true "(R=0.000000,G=0.076933,B=1.000000,A=1.000000)"))
    (Default|ObstacleLocation Other (.location _outhit) (.distance _outhit))
    (for _array_element (Variables|RightHand-Obstacles|Getobstacles)
      (if (> (Variables|Default|Getmin) (Variables|/Game/Minjeong/Actor/BP_NewParentObstacle.BP_NewParentObstacle_C|GetDistance _array_element))
        (bind _output_get_2 (Variables|RightHand-Obstacles|SettargetObstacle _array_element))
        (bind _output_get_3 (Variables|RightHand-Obstacles|SetnowObstacle _output_get_2))
        (Variables|RightHand-Hit|SethitRight (Variables|/Game/Minjeong/Actor/BP_NewParentObstacle.BP_NewParentObstacle_C|GetLocation _output_get_3))
        (Variables|Default|Setmin (Variables|/Game/Minjeong/Actor/BP_NewParentObstacle.BP_NewParentObstacle_C|GetDistance _output_get_3))))
    (if (!= (Variables|RightHand-Obstacles|GetprevObstacle) (Variables|RightHand-Obstacles|GetnowObstacle)) ; If we update the obstacle for a new one, we make colliderChanged TRUE
      (bind _output_get_4 (Variables|RightHand-Obstacles|SetcolliderChanged true))
      (Variables|RightHand-Obstacles|SetprevObstacle (Variables|RightHand-Obstacles|GetnowObstacle)))
    (Utilities|FlowControl|Sequence
      (:then_0
        ;[1 1 1] When do we update?
        (if (Variables|RightHand-Debug|GethasRightStartedMovingIn) ; 1. We update constantly to the hit if we did not reach yet the position or if we stop being in contact when the distance to the hit is larger than the arm itself\n2. Otherwise, hasLeftStartedMovingIn is false
          (bind _offset (CallFunction|SetOffset))
          (bind _output_get_5 (Variables|Default|Setoffset _offset))
          (Variables|RightHand-Hit|SethitRightFixed (+ (Variables|RightHand-Hit|GethitRight) _output_get_5))
          (Variables|RightHand-Hit|SetlocalHitRightFixed (- (Variables|RightHand-Hit|GethitRightFixed) (Variables|EventParam|GetPositionStay)))
          (else
            (switch Utilities|FlowControl|Switch|SwitchonE_ObstacleTag (.Tag (Utilities|Struct|BreakS_Obstacle _s_obstacle)) ; Two types of objects: Dynamic and Static
              (:NewEnumerator0
                (bind _offset_2 (CallFunction|SetOffset))
                (Variables|Default|Setoffset _offset_2)
                (if (Variables|RightHand-IK|GetfixHandToDynamicObject)
                  (Variables|RightHand-Hit|SethitRightFixed (+ (Variables|EventParam|GetPositionStay) (Variables|RightHand-Hit|GetlocalHitRightFixed) (Variables|Default|Getoffset)))
                  (elif (not (and (not (Variables|RightHand-Obstacles|GetcolliderChanged)) (not (Variables|RightHand-Debug|GethasRightStartedMovingIn)))) ; During the contact, we update constantly to the hit\nIf the system detects a change of obstacle, we update the bools, that will induce again the smooth transition
                    ;;[1 1 1] // Start moving to the target
                    (if (Variables|RightHand-Obstacles|GetcolliderChanged)
                      (Variables|RightHand-Debug|SethasRightStartedMovingIn true)
                      (Variables|RightHand-Debug|SethasRightTargetReached false)
                      (Variables|RightHand-Debug|SethasRightStartedMovingOut false)))))
              (:NewEnumerator1
                (if (not (Variables|Default|GetisLeftInRange))
                  (bind _offset_3 (CallFunction|SetOffset))
                  (Variables|Default|Setoffset _offset_3)))))))
      (:then_1
        ;[1 1 1] Debug Draw Ray : Launch a ray from the body part to protect, in the direction the closest point (like in the previous red ray)
        (if (Variables|RightHand-IK|GetdrawIK)
          (Collision|LineTraceByChannel (.location (Variables|Default|GetoriginRightRegion)) (Variables|RightHand-Hit|GethitRightFixed) "TraceTypeQuery1" false 0 "None" true "(R=1.000000,G=0.000000,B=0.844624,A=1.000000)" "(R=0.000000,G=0.075514,B=1.000000,A=1.000000)")))
      (:then_2))))

(event Custom|OnTriggerEndEvent
  (params (Other :type BP%20New%20Parent%20Obstacle%20Object%20Reference) (Positon :type Vector) (ID :type Integer))
  (Variables|EventParam|SetPositonEnd Positon)
  (bind _s_obstacle (CallFunction|ObstacleIDtoStruct ID))
  (if (Utilities|Enum|NotEqual(Enum) (.Tag (Utilities|Struct|BreakS_Obstacle _s_obstacle)) "NewEnumerator2")
    (Utilities|Array|RemoveItem (Variables|RightHand-Obstacles|Getobstacles) Other))
  (if (== (Utilities|Array|Length (Variables|RightHand-Obstacles|Getobstacles)) 0)
    ;[1 1 1] // Starts moving out
    (bind _output_get (Variables|RightHand-Debug|SethasRightStartedMovingIn false))
    (bind _output_get_2 (Variables|RightHand-Debug|SethasRightTargetReached false))
    (bind _output_get_3 (Variables|RightHand-Debug|SethasRightStartedMovingOut true))
    (Variables|Default|Setmin 1e+02)))
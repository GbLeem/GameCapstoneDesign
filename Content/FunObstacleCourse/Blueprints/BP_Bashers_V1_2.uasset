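; BP_Bashers_V1_2 is an obstacle course piece with four moving pillars.
; On BeginPlay, a Sequence starts four separate timelines, one per pillar.
; Each timeline's Location track drives its pillar's relative Y position on every update, while X stays fixed, placing two pillars on each side of the actor origin.
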(event EventBeginPlay
  (Utilities|FlowControl|Sequence
    (:then_0
      (bind _location (Timeline|Timeline_2 PlayFromStart)
        (:Update
          (Transformation|SetRelativeLocation (Variables|Default|GetPillar_2) (Math|Vector|MakeVector -1e+02 _location 0.0) false false))))
    (:then_1
      (bind _location_2 (Timeline|Timeline_0 PlayFromStart)
        (:Update
          (Transformation|SetRelativeLocation (Variables|Default|GetPillar_23) (Math|Vector|MakeVector 1e+02 _location_2 0.0) false false))))
    (:then_2
      (bind _location_3 (Timeline|Pillar3_Location PlayFromStart)
        (:Update
          (Transformation|SetRelativeLocation (Variables|Default|GetPillar_22) (Math|Vector|MakeVector 1e+02 _location_3 0.0) false false))))
    (:then_3
      (bind _location_4 (Timeline|Timeline_1 PlayFromStart)
        (:Update
          (Transformation|SetRelativeLocation (Variables|Default|GetPillar_21) (Math|Vector|MakeVector -1e+02 _location_4 0.0) false false))))))

(fn ConstructionScript)